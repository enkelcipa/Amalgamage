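; Tower exterior effects actor that cycles two particle systems on a repeating schedule.
; BeginPlay starts a looping timer that calls FireFX every seven seconds and stores its handle.
; FireFX activates the first particle system, swaps to the second after a short delay, then deactivates that one after an equal delay, leaving a brief gap before the next cycle.
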(event Custom|FireFX
  (bind _particlesystem (Variables|Default|GetParticleSystem))
  (bind _particlesystem1 (Variables|Default|GetParticleSystem1))
  (Components|Activation|Activate _particlesystem false)
  (Utilities|FlowControl|Delay 2.5)
  (Components|Activation|Deactivate _particlesystem)
  (Components|Activation|Activate _particlesystem1 false)
  (Utilities|FlowControl|Delay 2.5)
  (Components|Activation|Deactivate _particlesystem1))

(event EventBeginPlay
  (bind _returnvalue (Utilities|Time|SetTimerbyEvent (delegate Custom|FireFX) 7.0 true))
  (Variables|Default|SetTimer _returnvalue))

(fn ConstructionScript)