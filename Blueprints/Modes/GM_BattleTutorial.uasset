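; Battle tutorial game mode that scripts a simplified fight on top of a parent battle mode's turn and round flow.
; BeginPlay resets TurnCount and spawns a fire blob and an enemy before running the parent logic.
; Round starts check TurnCount to add, once each, a water blob and then another enemy.
; Every new turn disables the HUD's action button after the parent turn logic runs.
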(event EventBeginPlay
  (Variables|Default|SetTurnCount 0)
  (CallFunction|SpawnUnit :UnitToSpawn "BlobFire" :Position 1)
  (CallFunction|SpawnUnit :UnitToSpawn "Enemy3" :Position 1 :bEnemy true)
  (|CallParentFunction))

(event EventStartNextTurn
  (|CallParentFunction)
  (Widget|SetIsEnabled (Variables|/Game/UI/WBP_Actions.WBP_Actions_C|GetActionButtonREF (Variables|/Game/UI/WBP_HUD.WBP_HUD_C|GetWBP_Actions (Variables|Default|GetHUDRef))) false))

(event EventStartNextRound
  (|CallParentFunction)
  (if (== (Variables|Default|GetTurnCount) 1)
    (Utilities|FlowControl|DoOnce false
      (:Completed
        (CallFunction|SpawnUnit :UnitToSpawn "BlobWater")))
    (elif (== (Variables|Default|GetTurnCount) 2)
      (Utilities|FlowControl|DoOnce false
        (:Completed
          (CallFunction|SpawnUnit :Position 1 :bEnemy true))))))

(fn ConstructionScript
  (|CallParentFunction))