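; PC_Battle is the battle player controller that relays player input to the GM_Battle game mode.
; On BeginPlay it caches the game mode and adds the Enhanced Input mapping context.
; Click sends the actor under the cursor, found by an object-type trace, to the game mode, and pause is forwarded likewise.
; A ChangeSelection helper steps the selected unit index and notifies the game mode, but its only call here is unwired, alongside leftover test nodes.
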(event Input|EnhancedActionEvents|EnhancedInputActionIA_Click
  (params (ActionValue :type Boolean) (ElapsedSeconds :type Float%20%28double-precision%29) (TriggeredSeconds :type Float%20%28double-precision%29) (InputAction :type Input%20Action%20Object%20Reference :default "/Game/Input/IA_Click.IA_Click"))
  (:Started
    (Class|BPIControls|LeftClickAction(Message) (Variables|Default|GetGameModeREF) false "NewEnumerator1" (.HitActor (Collision|BreakHitResult (.HitResult (Class|PlayerController|GetHitResultUnderCursorforObjects (Variables|Default|GetObject%20Types) true)))))))

(event Input|EnhancedActionEvents|EnhancedInputActionIA_Pause
  (params (ActionValue :type Boolean) (ElapsedSeconds :type Float%20%28double-precision%29) (TriggeredSeconds :type Float%20%28double-precision%29) (InputAction :type Input%20Action%20Object%20Reference :default "/Game/Input/IA_Pause.IA_Pause"))
  (:Started
    (Default|PausePressed (Variables|Default|GetGameModeREF) false "NewEnumerator1")))

(event EventBeginPlay
  (bind _asgm_battle (Utilities|Casting|CastToGM_Battle (Game|GetGameMode)))
  (Variables|Default|SetGameModeREF _asgm_battle)
  (Input|AddMappingContext (PlayerController|LocalPlayerSubsystems|GetEnhancedInputLocalPlayerSubsystem self) "/Game/Input/IMC_Controlls.IMC_Controlls" 0 "(bIgnoreAllPressedKeysUntilRelease=True,bForceImmediately=False,bNotifyUserSettings=False)"))

(event EventTick
  (params (DeltaSeconds :type Float%20%28single-precision%29)))

(event Input|KeyboardEvents|DebugKey1
  (params (Key :type Key%20Structure :default "None") (ActionValue :type Input%20Action%20Value%20Structure)))

(event Input|KeyboardEvents|DebugKeyF
  (params (Key :type Key%20Structure :default "None") (ActionValue :type Input%20Action%20Value%20Structure)))

(event Input|KeyboardEvents|DebugKeyG
  (params (Key :type Key%20Structure :default "None") (ActionValue :type Input%20Action%20Value%20Structure)))

(event Input|KeyboardEvents|DebugKey2
  (params (Key :type Key%20Structure :default "None") (ActionValue :type Input%20Action%20Value%20Structure)))

(fn ConstructionScript)

(fn ChangeSelection
  (params (bForwards :type Boolean))
  (bind _output_get (Variables|Default|SetSelectedUnit (+ (Variables|Default|GetSelectedUnit) (Math|Integer|SelectInt 1 -1 bForwards))))
  (Default|CallOnSelectionChanged (Variables|Default|GetGameModeREF) _output_get)
  (return _output_get))