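; BP_SummoningCandles is a set of three summoning candles that shows how many are lit, from none to all three.
; ToggleCandlelight switches on CandleIndex and sets the visibility of each candle's light, flame and smoke components, lighting candles cumulatively in order.
; Each case writes the full state of all three candles, and the event's caller is outside this Blueprint.
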(event EventToggleCandlelight
  (params (CandleIndex :type Integer))
  (switch int CandleIndex
    (:0
      (Rendering|SetVisibility (Variables|Default|GetCandle1_Light1) false false)
      (Rendering|SetVisibility (Variables|Default|GetCandle2_Light1) false false)
      (Rendering|SetVisibility (Variables|Default|GetCandle3_Light1) false false))
    (:1
      (Rendering|SetVisibility (Variables|Default|GetCandle1_Light1) true false)
      (Rendering|SetVisibility (Variables|Default|GetCandle2_Light1) false false)
      (Rendering|SetVisibility (Variables|Default|GetCandle3_Light1) false false))
    (:2
      (Rendering|SetVisibility (Variables|Default|GetCandle1_Light1) true false)
      (Rendering|SetVisibility (Variables|Default|GetCandle2_Light1) true false)
      (Rendering|SetVisibility (Variables|Default|GetCandle3_Light1) false false))
    (:3
      (Rendering|SetVisibility (Variables|Default|GetCandle1_Light1) true false)
      (Rendering|SetVisibility (Variables|Default|GetCandle2_Light1) true false)
      (Rendering|SetVisibility (Variables|Default|GetCandle3_Light1) true false))))

(fn ConstructionScript)