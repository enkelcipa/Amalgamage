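; BP_SelectManager is the main menu manager that holds the selectable unit list and original camera for the selection HUD.
; On BeginPlay it refreshes each unit's data from DT_Units by name, snapshots the list, then registers itself with the HUD from GM_MainMenu after a short delay.
; ResetList restores the snapshot and updates the selection HUD.
; RemoveBlob is an empty event, with removal logic left disconnected.
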(event Custom|RemoveBlob
  (params (Blob :type BP%20Base%20Unit%20Object%20Reference) (SelectionHUD :type WBP%20Blob%20Selection%20HUD%20Object%20Reference)))

(event Custom|ResetList
  (params (SelectionHUD :type WBP%20Blob%20Selection%20HUD%20Object%20Reference))
  (bind _output_get (Variables|Default|SetUnits (Variables|Default|GetOriginalUnits)))
  (Default|UpdateMe SelectionHUD _output_get false))

(event EventBeginPlay
  (for _array_element (Variables|Default|GetUnits)
    (bind _returnvalue (Utilities|GetDataTableRow "/Game/Blueprints/Data/DT_Units.DT_Units" (Utilities|String|StringToName (Utilities|String|ToString(Text) (.Name (Utilities|Struct|BreakStruct_UnitData (Variables|/Game/Blueprints/Units/BP_BaseUnit.BP_BaseUnit_C|GetUnitData _array_element))))))
      (:then
        (Variables|/Game/Blueprints/Units/BP_BaseUnit.BP_BaseUnit_C|SetUnitData _array_element _returnvalue))))
  (Variables|Default|SetOriginalUnits (Variables|Default|GetUnits))
  (bind _asgm_main_menu (Utilities|Casting|CastToGM_MainMenu (Game|GetGameMode)))
  (bind _output_get (Variables|Default|SetGameModeREF _asgm_main_menu))
  (Utilities|FlowControl|Delay 0.2)
  (bind _hud (Default|GetHUDREF _output_get))
  (bind _output_get_2 (Variables|Default|SetHUDREF _hud))
  (Default|GiveManagerREF _output_get_2 self))

(fn ConstructionScript)

(fn GetUnitREFs
  (return (Variables|Default|GetUnits)))

(fn GetOriginalCamera
  (return (Variables|Default|GetOriginalCamera)))