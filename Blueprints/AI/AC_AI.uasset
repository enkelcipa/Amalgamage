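; Enemy AI component for turn-based battles that picks an action and target for the acting unit through utility scoring.
; AIBegin filters out dead units, then branches: Water/Earth units support low-HP allies, others focus a target with three Overcharge stacks, or else Nature/Lightning units weigh debuffs against basic attacks.
; Formulas score action-target pairs on elemental priority, HP, enemy mana, existing statuses and some randomness; PickTarget selects the highest.
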(event EventBeginPlay)

(event EventTick
  (params (DeltaSeconds :type Float%20%28single-precision%29)))

(fn AIBegin
  (params (Actions :type Array%20of%20BP%20Base%20Action%20Class%20References) (Player%20Units :type Array%20of%20BP%20Base%20Unit%20Object%20References) (AI%20Units :type Array%20of%20BP%20Base%20Unit%20Object%20References) (This%20Unit :type BP%20Base%20Unit%20Object%20Reference))
  (bind (_living_ai_units _living_player_units) (CallFunction|RemoveDeadUnitsfromTargeting AI%20Units Player%20Units))
  (LocalVariables|SetLiving%20AI%20Units _living_ai_units)
  (LocalVariables|SetLiving%20Player%20Units _living_player_units)
  (LocalVariables|SetBasic%20Attack (Utilities|Array|Get(acopy) Actions (Utilities|Array|FindItem Actions "/Game/Blueprints/Actions/BP_BasicAttack.BP_BasicAttack_C")))
  (Utilities|Array|Clear (Variables|Default|GetAll%20Possible%20Options))
  ;[0.15 0.15 0.15 0.5] Am I a healer or not?
  (bind (_healer_ _support_ability) (Healer|DoIHaveASupportiveAbility? This%20Unit))
  (if _healer_
    ;[0.15 0.15 0.15 0.5] Do I need to heal?
    (bind _heal_ (Healer|DoINeedtoHeal/Support? (LocalVariables|GetLiving%20AI%20Units)))
    (if _heal_
      ;[0.15 0.15 0.15 0.5] Run Healing Formula
      (bind _chosen_option (Healer|Healing/SupportFormula (LocalVariables|GetLiving%20AI%20Units) _support_ability))
      ;[0.15 0.15 0.15 0.5] Heal chosen target
      (return (.ChosenAction (Utilities|Struct|BreakS_AIDecision _chosen_option)) (.Target (Utilities|Struct|BreakS_AIDecision _chosen_option)))
      (else
        ;[0.15 0.15 0.15 0.5] Run Basic Attack Formula
        (bind _chosen_option_2 (CallFunction|BasicAttackFormula (Utilities|Array|MakeArray (LocalVariables|GetBasic%20Attack)) (LocalVariables|GetLiving%20Player%20Units) false))
        ;[0.15 0.15 0.15 0.5] Attack chosen target
        (return (.ChosenAction (Utilities|Struct|BreakS_AIDecision _chosen_option_2)) (.Target (Utilities|Struct|BreakS_AIDecision _chosen_option_2)))))
    (else
      ;[0.15 0.15 0.15 0.5] Does any target have 3 lightning stacks?
      (bind (_chosen_option_3 _am_i_detonating_stacks_) (CallFunction|CheckLightningStacks (LocalVariables|GetLiving%20Player%20Units)))
      ;[0.15 0.15 0.15 0.5] Am I detonating stacks?
      (if _am_i_detonating_stacks_
        (bind _chosen_option_4 (CallFunction|BasicAttackFormula Actions (Utilities|Array|MakeArray (Utilities|Struct|BreakS_AIDecision _chosen_option_3)) false))
        ;[0.15 0.15 0.15 0.5] Attack that target
        (return (.ChosenAction (Utilities|Struct|BreakS_AIDecision _chosen_option_4)) (.Target (Utilities|Struct|BreakS_AIDecision _chosen_option_4)))
        (else
          ;[0.15 0.15 0.15 0.5] Am I a debuffer?
          (bind (_debuffer_ _debuff) (Debuffer|DoIHaveDebuffs? This%20Unit))
          (if _debuffer_
            ;[0.15 0.15 0.15 0.5] Run Debuff Formula
            (Debuffer|DebuffingFormula (LocalVariables|GetLiving%20Player%20Units) _debuff)
            ;[0.15 0.15 0.15 0.5] Run Basic Attack Formula
            (CallFunction|BasicAttackFormula (Utilities|Array|MakeArray (LocalVariables|GetBasic%20Attack)) (LocalVariables|GetLiving%20Player%20Units) true)
            ;[0.15 0.15 0.15 0.5] Pick and execute action on chosen target
            (bind _chosen_option_5 (FormulaComponent|PickTarget (Variables|Default|GetAll%20Possible%20Options)))
            (return (.ChosenAction (Utilities|Struct|BreakS_AIDecision _chosen_option_5)) (.Target (Utilities|Struct|BreakS_AIDecision _chosen_option_5)))
            (else
              ;[0.15 0.15 0.15 0.5] Run Basic Attack Formula
              (bind _chosen_option_6 (CallFunction|BasicAttackFormula Actions (LocalVariables|GetLiving%20Player%20Units) false))
              ;[0.15 0.15 0.15 0.5] Attack chosen target
              (return (.ChosenAction (Utilities|Struct|BreakS_AIDecision _chosen_option_6)) (.Target (Utilities|Struct|BreakS_AIDecision _chosen_option_6))))))))))

(fn BasicAttackFormula
  (params (Actions :type Array%20of%20BP%20Base%20Action%20Class%20References) (Potential%20Targets :type Array%20of%20BP%20Base%20Unit%20Object%20References) (Debuffer? :type Boolean))
  (for _array_element Actions
    (bind _output_get (LocalVariables|SetT%20Action%20Choice _array_element))
    (for _array_element_2 Potential%20Targets
      (bind _target_priority (FormulaComponent|CalculateTargetPriority _array_element_2))
      (bind _hp_urgency (FormulaComponent|CalculateHPUrgency _array_element_2))
      (bind _mana_score (FormulaComponent|CalculateManaScore (Utilities|Struct|BreakStruct_ActionData (Utilities|GetClassDefaults _output_get))))
      (Utilities|Array|Add (Variables|Default|GetAll%20Possible%20Options) (Utilities|Struct|MakeS_AIDecision (LocalVariables|GetT%20Action%20Choice) _array_element_2 (|((((BaseScore+TargetPriority)-HPUrgency)+MPCost)+Random) 2e+01 _target_priority _hp_urgency _mana_score (Math|Random|RandomFloatinRange 0.0 15.0))))))
  (if (not Debuffer?)
    (bind _chosen_option (FormulaComponent|PickTarget (Variables|Default|GetAll%20Possible%20Options)))
    (return _chosen_option)))

(fn CalculateTargetPriority
  (params (Potential%20Target :type BP%20Base%20Unit%20Object%20Reference))
  (LocalVariables|SetPriority%20Score 0.0)
  (for _array_element (Utilities|Struct|BreakStruct_UnitData (Variables|/Game/Blueprints/Units/BP_BaseUnit.BP_BaseUnit_C|GetUnitData Potential%20Target))
    (LocalVariables|SetPriority%20Score (+ (LocalVariables|GetPriority%20Score) (.Value (Utilities|Map|Find (LocalVariables|GetElemental%20Priority) _array_element)))))
  (return (LocalVariables|GetPriority%20Score)))

(fn CalculateHPUrgency
  (params (Potential%20Target :type BP%20Base%20Unit%20Object%20Reference))
  (bind _unitstats (Variables|/Game/Blueprints/Units/BP_BaseUnit.BP_BaseUnit_C|GetUnitStats Potential%20Target))
  (bind (_maxhp _currenthp) (Utilities|Struct|BreakStruct_UnitStats _unitstats))
  (return (|((CurHP/MaxHP)*10) (Math|Conversions|ToFloat(Integer) _currenthp) (Math|Conversions|ToFloat(Integer) _maxhp))))

(fn PickTarget
  (params (All%20Possible%20Actions :type Array%20of%20S%20AI%20Decision%20Structures))
  (LocalVariables|SetHighest%20Index 0)
  (LocalVariables|SetHighest%20Action%20Score 0.0)
  (for (_array_element _array_index) All%20Possible%20Actions
    (if (> (Utilities|Struct|BreakS_AIDecision _array_element) (LocalVariables|GetHighest%20Action%20Score))
      (LocalVariables|SetHighest%20Action%20Score (Utilities|Struct|BreakS_AIDecision _array_element))
      (LocalVariables|SetHighest%20Index _array_index)))
  (return (Utilities|Array|Get(acopy) All%20Possible%20Actions (LocalVariables|GetHighest%20Index))))

(fn DoIHaveASupportiveAbility?
  (params (This%20Unit :type BP%20Base%20Unit%20Object%20Reference))
  (bind _unitdata (Variables|/Game/Blueprints/Units/BP_BaseUnit.BP_BaseUnit_C|GetUnitData This%20Unit))
  (bind _baseaffinities (Utilities|Struct|BreakStruct_UnitData _unitdata))
  (if (or (Utilities|Array|ContainsItem _baseaffinities "NewEnumerator1") (Utilities|Array|ContainsItem _baseaffinities "NewEnumerator2"))
    (switch Utilities|FlowControl|Switch|SwitchoneElement (Utilities|Array|Get(acopy) (.BaseAffinities (Utilities|Struct|BreakStruct_UnitData (Variables|/Game/Blueprints/Units/BP_BaseUnit.BP_BaseUnit_C|GetUnitData This%20Unit))))
      (:NewEnumerator1
        (return true "/Game/Blueprints/Actions/BP_Heal.BP_Heal_C"))
      (:NewEnumerator2
        (return true "/Game/Blueprints/Actions/BP_ShieldCast.BP_ShieldCast_C")))
    (else
      (return false 0))))

(fn DoINeedtoHeal/Support?
  (params (AI%20Units :type Array%20of%20BP%20Base%20Unit%20Object%20References))
  (for _array_element AI%20Units
    (bind _target_hp_ (CallFunction|CalculateTargetHP% _array_element))
    (if (<= _target_hp_ 25.0)
      (return true)))
  (return false))

(fn Healing/SupportFormula
  (params (AI%20Units :type Array%20of%20BP%20Base%20Unit%20Object%20References) (Support%20Action :type BP%20Base%20Ability%20Class%20Reference))
  (Utilities|Array|Clear (LocalVariables|GetPotential%20Targets%20to%20Heal))
  (for _array_element AI%20Units
    (bind _target_hp_ (CallFunction|CalculateTargetHP% _array_element))
    (if (<= _target_hp_ 25.0)
      (Utilities|Array|Add (LocalVariables|GetPotential%20Targets%20to%20Heal) _array_element)))
  (for _array_element_2 (LocalVariables|GetPotential%20Targets%20to%20Heal)
    (bind _hp_urgency (FormulaComponent|CalculateHPUrgency _array_element_2))
    (bind _mana_score (FormulaComponent|CalculateManaScore (Utilities|Struct|BreakStruct_ActionData (Utilities|GetClassDefaults Support%20Action))))
    (Utilities|Array|Add (Variables|Default|GetAll%20Possible%20Options) (Utilities|Struct|MakeS_AIDecision Support%20Action _array_element_2 (|(((BaseScore-HPUrgency)+MPCost)+Random) 2e+01 _hp_urgency _mana_score (Math|Random|RandomFloatinRange 0.0 1e+01)))))
  (bind _chosen_option (FormulaComponent|PickTarget (Variables|Default|GetAll%20Possible%20Options)))
  (return _chosen_option))

(fn CalculateTargetHP%
  (params (Target :type BP%20Base%20Unit%20Object%20Reference))
  (bind _unitstats (Variables|/Game/Blueprints/Units/BP_BaseUnit.BP_BaseUnit_C|GetUnitStats Target))
  (bind (_maxhp _currenthp) (Utilities|Struct|BreakStruct_UnitStats _unitstats))
  (return (|((CurHP/MaxHP)*100) (Math|Conversions|ToFloat(Integer) _currenthp) (Math|Conversions|ToFloat(Integer) _maxhp))))

(fn CheckLightningStacks
  (params (Player%20Units :type Array%20of%20BP%20Base%20Unit%20Object%20References))
  (bind _player_and_no__stacks (LocalVariables|GetPlayer%20and%20No.%20Stacks))
  ;[0.15 0.15 0.15 0.5] Clear temp variables
  (Utilities|Map|Clear (LocalVariables|GetPlayer%20and%20No.%20Stacks))
  (LocalVariables|SetTemp%20Stack%20Quant 0)
  ;[0.15 0.15 0.15 0.5] Check for lightning status and quantities
  (for _array_element Player%20Units
    (for _array_element_2 (Actor|GetAttachedActors _array_element true false)
      (bind _asbp_status_overcharge (Utilities|Casting|CastToBP_StatusOvercharge _array_element_2))
      (Utilities|Map|Add (LocalVariables|GetPlayer%20and%20No.%20Stacks) _array_element (Variables|/Game/Blueprints/Statuses/BP_StatusOvercharge.BP_StatusOvercharge_C|GetStacks _asbp_status_overcharge))))
  (bind _values (Utilities|Map|Values _player_and_no__stacks))
  (if (<= (.MaxValue (Math|Integer|MaxOfIntArray _values)) 2)
    (return "" false)
    (else
      (return (Utilities|Struct|MakeS_AIDecision (.Key (Utilities|Map|GetKeyValueByIndex _player_and_no__stacks (.IndexOfMaxValue (Math|Integer|MaxOfIntArray _values))))) true))))

(fn DoIHaveDebuffs?
  (params (This%20Unit :type BP%20Base%20Unit%20Object%20Reference))
  (bind _unitdata (Variables|/Game/Blueprints/Units/BP_BaseUnit.BP_BaseUnit_C|GetUnitData This%20Unit))
  (bind _baseaffinities (Utilities|Struct|BreakStruct_UnitData _unitdata))
  (if (or (Utilities|Array|ContainsItem _baseaffinities "NewEnumerator3") (Utilities|Array|ContainsItem _baseaffinities "NewEnumerator4"))
    (switch Utilities|FlowControl|Switch|SwitchoneElement (Utilities|Array|Get(acopy) (.BaseAffinities (Utilities|Struct|BreakStruct_UnitData (Variables|/Game/Blueprints/Units/BP_BaseUnit.BP_BaseUnit_C|GetUnitData This%20Unit))))
      (:NewEnumerator3
        (return true "/Game/Blueprints/Actions/BP_Entangle.BP_Entangle_C"))
      (:NewEnumerator4
        (return true "/Game/Blueprints/Actions/BP_Overcharge.BP_Overcharge_C")))
    (else
      (return false 0))))

(fn DebuffingFormula
  (params (Player%20Units :type Array%20of%20BP%20Base%20Unit%20Object%20References) (Debuffing%20Ability :type BP%20Base%20Ability%20Class%20Reference))
  (if (== Debuffing%20Ability "/Game/Blueprints/Actions/BP_Overcharge.BP_Overcharge_C")
    ;[0.15 0.15 0.15 0.5] Check each player unit and count their stacks. Factor stacks into Action Score
    (for _array_element Player%20Units
      (LocalVariables|SetTemp%20Stack%20Quant 0.0)
      (for _array_element_2 (Actor|GetAttachedActors _array_element true false)
        (bind _asbp_status_overcharge (Utilities|Casting|CastToBP_StatusOvercharge _array_element_2))
        (if (< (Variables|/Game/Blueprints/Statuses/BP_StatusOvercharge.BP_StatusOvercharge_C|GetStacks _asbp_status_overcharge) 3)
          (LocalVariables|SetTemp%20Stack%20Quant 5.0)
          (else
            (LocalVariables|SetTemp%20Stack%20Quant -5.0))))
      (bind _mana_score (FormulaComponent|CalculateManaScore (Utilities|Struct|BreakStruct_ActionData (Utilities|GetClassDefaults Debuffing%20Ability))))
      (Utilities|Array|Add (Variables|Default|GetAll%20Possible%20Options) (Utilities|Struct|MakeS_AIDecision Debuffing%20Ability _array_element (|(((BaseScore+StackAmount)+MPCost)+Random) 2e+01 (LocalVariables|GetTemp%20Stack%20Quant) _mana_score (Math|Random|RandomFloatinRange 0.0 0.0)))))
    (else
      ;[0.15 0.15 0.15 0.5] Check each player unit for entange. Reduces score to reduce chance of adding it again
      (for _array_element_3 Player%20Units
        (LocalVariables|SetHas%20Entange 3)
        (for _array_element_4 (Actor|GetAttachedActors _array_element_3 true false)
          (if (== (Utilities|GetClass _array_element_4) "/Game/Blueprints/Actions/BP_Entangle.BP_Entangle_C")
            (Utilities|NegateInt (LocalVariables|GetHas%20Entange))
            (else
              (Math|Integer|IncrementInt (LocalVariables|GetHas%20Entange)))))
        (bind _mana_score_2 (FormulaComponent|CalculateManaScore (Utilities|Struct|BreakStruct_ActionData (Utilities|GetClassDefaults Debuffing%20Ability))))
        (Utilities|Array|Add (Variables|Default|GetAll%20Possible%20Options) (Utilities|Struct|MakeS_AIDecision Debuffing%20Ability _array_element_3 (|(((BaseScore-HasEntangle)+MPCost)+Random) 2e+01 (Math|Conversions|ToFloat(Integer) (* (LocalVariables|GetHas%20Entange) 5)) _mana_score_2 (Math|Random|RandomFloatinRange 0.0 0.0))))))))

(fn CalculateManaScore
  (params (Mana%20Cost :type Integer))
  (bind _asgm_battle (Utilities|Casting|CastToGM_Battle (Game|GetGameMode)))
  (if (< (* Mana%20Cost 1.05) (Variables|/Game/Blueprints/Modes/GM_Battle.GM_Battle_C|GetCurrentEnemyMana _asgm_battle))
    (return 1e+01)
    (else
      (return -1e+01))))

(fn RemoveDeadUnitsfromTargeting
  (params (AI%20Units :type Array%20of%20BP%20Base%20Unit%20Object%20References) (Player%20Units :type Array%20of%20BP%20Base%20Unit%20Object%20References))
  (LocalVariables|SetTemp%20AI%20Units AI%20Units)
  (LocalVariables|SetTemp%20Player%20Units Player%20Units)
  (for _array_element AI%20Units
    (if (Variables|/Game/Blueprints/Units/BP_BaseUnit.BP_BaseUnit_C|GetDead _array_element)
      (Utilities|Array|RemoveItem (LocalVariables|GetTemp%20AI%20Units) _array_element)))
  (for _array_element_2 Player%20Units
    (if (Variables|/Game/Blueprints/Units/BP_BaseUnit.BP_BaseUnit_C|GetDead _array_element_2)
      (Utilities|Array|RemoveItem (LocalVariables|GetTemp%20Player%20Units) _array_element_2)))
  (return (LocalVariables|GetTemp%20AI%20Units) (LocalVariables|GetTemp%20Player%20Units)))