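; Overcharge status effect that stacks on a unit and detonates as a lightning burst through the unit's deal-damage event.
; Each application increments TurnsRemaining, used as a stack count since TickStatus is empty, and broadcasts it.
; Detonate plays effects, then deals base plus percent-of-max-HP damage scaled for one to three stacks, and expires the status.
; A DoOnce limits the damage to one trigger, though effects play before it.
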(event Custom|Detonate
  (params (Caster :type BP%20Base%20Unit%20Object%20Reference) (Amount :type Integer))
  (Niagara|SpawnSystematLocation "/Game/VFX/ElementalVFX/NS_Lightning.NS_Lightning" (+ (Transformation|GetActorLocation (Variables|Default|GetUnit)) "0.000000,0.000000,50.000000"))
  (Audio|PlaySound2D "/Game/Audio/Magic_Spell_SFX_Pack_Vol1/Lightning/cue/Lightning_Magic_Spell_9-1_wav_Cue.Lightning_Magic_Spell_9-1_wav_Cue" 1.0 1.0 0.0 0 0)
  (Variables|Default|SetMax%20HP (Utilities|Struct|BreakStruct_UnitStats (Variables|/Game/Blueprints/Units/BP_BaseUnit.BP_BaseUnit_C|GetUnitStats (Variables|Default|GetUnit))))
  (Utilities|FlowControl|DoOnce false
    (:Completed
      (switch int (Variables|Default|GetTurnsRemaining)
        (:1
          (Variables|Default|SetDamage (Math|Float|Round (|(Base+(MaxHP*PercentDMG)) 3.0 (Math|Conversions|ToFloat(Integer) (Variables|Default|GetMax%20HP)) 0.03))))
        (:2
          (Variables|Default|SetDamage (Math|Float|Round (|(Base+(MaxHP*PercentDMG)) 1e+01 (Math|Conversions|ToFloat(Integer) (Variables|Default|GetMax%20HP)) 0.15))))
        (:3
          (Variables|Default|SetDamage (Math|Float|Round (|(Base+(MaxHP*PercentDMG)) 2e+01 (Math|Conversions|ToFloat(Integer) (Variables|Default|GetMax%20HP)) 0.25)))))
      (Default|DealDamage (Variables|Default|GetUnit) (Variables|Default|GetDamage) (Utilities|Map|MakeMap "NewEnumerator4" 1.0) 0 false)
      (CallFunction|StatusExpired))))

(event EventBeginPlay
  (|CallParentFunction)
  (CallFunction|ApplyEffects)
  (EventDispatchers|BindEventtoOnDealDamage (Variables|Default|GetUnit) (EventDispatchers|CreateEvent :!event Custom|Detonate)))

(event Collision|EventActorBeginOverlap
  (params (OtherActor :type Actor%20Object%20Reference))
  (|CallParentFunction OtherActor) ; This node is disabled and will not be called.\nDrag off pins to build functionality.
)

(event EventTick
  (params (DeltaSeconds :type Float%20%28single-precision%29))
  (|CallParentFunction DeltaSeconds) ; This node is disabled and will not be called.\nDrag off pins to build functionality.
)

(event EventApplyEffects
  (|CallParentFunction)
  (bind _result (Math|Integer|IncrementInt (Variables|Default|GetTurnsRemaining))
    (:%20%20
      (Default|CallOnOverchargeApplied _result))))

(event EventTickStatus)

(fn ConstructionScript
  (|CallParentFunction))