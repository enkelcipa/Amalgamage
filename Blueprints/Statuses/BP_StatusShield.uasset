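; BP_StatusShield is a unit status effect that makes its Unit invincible while it lasts.
; On BeginPlay it applies the effect by setting Invincible in the unit's stats and binds to the unit's OnHitBlocked event; clearing reverts the flag.
; IncrementShield and TickStatus raise or lower TurnsRemaining, which doubles as the shield count broadcast through OnShieldApplied.
; When a tick brings the count to zero, the status expires.
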(event EventBeginPlay
  (|CallParentFunction)
  (CallFunction|ApplyEffects)
  (EventDispatchers|BindEventtoOnHitBlocked (Variables|Default|GetUnit) (EventDispatchers|CreateEvent :!event TickStatus)))

(event Collision|EventActorBeginOverlap
  (params (OtherActor :type Actor%20Object%20Reference))
  (|CallParentFunction OtherActor) ; This node is disabled and will not be called.\nDrag off pins to build functionality.
)

(event EventTick
  (params (DeltaSeconds :type Float%20%28single-precision%29))
  (|CallParentFunction DeltaSeconds) ; This node is disabled and will not be called.\nDrag off pins to build functionality.
)

(event EventApplyEffects
  (|CallParentFunction)
  (Utilities|Struct|SetmembersinStruct_UnitStats (Variables|/Game/Blueprints/Units/BP_BaseUnit.BP_BaseUnit_C|GetUnitStats (Variables|Default|GetUnit)) true))

(event EventClearEffects
  (|CallParentFunction)
  (Utilities|Struct|SetmembersinStruct_UnitStats (Variables|/Game/Blueprints/Units/BP_BaseUnit.BP_BaseUnit_C|GetUnitStats (Variables|Default|GetUnit)) false))

(event EventTickStatus
  (bind _turnsremaining (Variables|Default|GetTurnsRemaining))
  (Math|Integer|DecrementInt (Variables|Default|GetTurnsRemaining)
    (:%20%20
      (Default|CallOnShieldApplied _turnsremaining)
      (if (<= _turnsremaining 0)
        (CallFunction|StatusExpired)))))

(event EventIncrementShield
  (Math|Integer|IncrementInt (Variables|Default|GetTurnsRemaining)
    (:%20%20
      (Default|CallOnShieldApplied (Variables|Default|GetTurnsRemaining)))))

(fn ConstructionScript
  (|CallParentFunction))