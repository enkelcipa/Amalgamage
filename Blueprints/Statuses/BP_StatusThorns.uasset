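; BP_StatusThorns is a thorns status effect that reflects a share of damage back at the caster who dealt it.
; On BeginPlay it runs the parent logic and binds an event to its Unit's OnDealDamage dispatcher.
; ApplyThornsDamage scales the incoming amount by ThornsDamage, rounds it and calls DealDamage on the Caster with the status's Types.
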(event Custom|Apply%20Thorns%20Damage
  (params (Caster :type BP%20Base%20Unit%20Object%20Reference) (Amount :type Integer))
  (Default|DealDamage Caster (Math|Float|Round (* (Math|Conversions|ToFloat(Integer) Amount) (Variables|Default|GetThorns%20%25%20Damage%20))) (Variables|Default|GetTypes) 0 false))

(event EventBeginPlay
  (|CallParentFunction)
  (EventDispatchers|BindEventtoOnDealDamage (Variables|Default|GetUnit) (EventDispatchers|CreateEvent :!event Custom|Apply%20Thorns%20Damage)))

(event Collision|EventActorBeginOverlap
  (params (OtherActor :type Actor%20Object%20Reference))
  (|CallParentFunction OtherActor) ; This node is disabled and will not be called.\nDrag off pins to build functionality.
)

(event EventTick
  (params (DeltaSeconds :type Float%20%28single-precision%29))
  (|CallParentFunction DeltaSeconds) ; This node is disabled and will not be called.\nDrag off pins to build functionality.
)

(fn ConstructionScript
  (|CallParentFunction))