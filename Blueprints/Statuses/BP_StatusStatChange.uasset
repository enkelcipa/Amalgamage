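; BP_StatusStatChange is a status actor that alters its Unit's attack, defence and speed modifiers.
; On BeginPlay it runs ApplyEffects, which adds its attack and defence modifiers into the Unit's UnitStats struct and passes its speed modifier to ModifySpeed.
; ClearEffects reverses this by subtracting the same amounts and calling ModifySpeed with the negated value.
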(event EventBeginPlay
  (|CallParentFunction)
  (CallFunction|ApplyEffects))

(event Collision|EventActorBeginOverlap
  (params (OtherActor :type Actor%20Object%20Reference))
  (|CallParentFunction OtherActor) ; This node is disabled and will not be called.\nDrag off pins to build functionality.
)

(event EventTick
  (params (DeltaSeconds :type Float%20%28single-precision%29))
  (|CallParentFunction DeltaSeconds) ; This node is disabled and will not be called.\nDrag off pins to build functionality.
)

(event EventApplyEffects
  (bind _unit (Variables|Default|GetUnit))
  (bind _unitstats (Variables|/Game/Blueprints/Units/BP_BaseUnit.BP_BaseUnit_C|GetUnitStats _unit))
  (bind (_attackmodifier _defensemodifier) (Utilities|Struct|BreakStruct_UnitStats _unitstats))
  (Utilities|Struct|SetmembersinStruct_UnitStats _unitstats (+ _attackmodifier (Variables|Default|GetAttack%20Modifier)) (+ _defensemodifier (Variables|Default|GetDefence%20Modifier)))
  (Default|ModifySpeed (Variables|Default|GetUnit) (Variables|Default|GetSpeed%20Modifier)))

(event EventClearEffects
  (bind _unit (Variables|Default|GetUnit))
  (bind _unitstats (Variables|/Game/Blueprints/Units/BP_BaseUnit.BP_BaseUnit_C|GetUnitStats _unit))
  (bind (_attackmodifier _defensemodifier) (Utilities|Struct|BreakStruct_UnitStats _unitstats))
  (Utilities|Struct|SetmembersinStruct_UnitStats _unitstats (- _attackmodifier (Variables|Default|GetAttack%20Modifier)) (- _defensemodifier (Variables|Default|GetDefence%20Modifier)))
  (Default|ModifySpeed (Variables|Default|GetUnit) (* (Variables|Default|GetSpeed%20Modifier) -1)))

(fn ConstructionScript
  (|CallParentFunction))