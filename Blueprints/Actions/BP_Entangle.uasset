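; BP_Entangle is a nature combat action that damages units and roots them with an Entangle status.
; On cast it spawns a nature aura effect above each target, plays a spell sound and starts a timeline.
; The timeline's Damage event hits every unit in the first target's AlliedUnits with damage and a timed BP_StatusEntangle, and its finish ends the action.
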(event EventBeginPlay
  (|CallParentFunction) ; This node is disabled and will not be called.\nDrag off pins to build functionality.
)

(event Collision|EventActorBeginOverlap
  (params (OtherActor :type Actor%20Object%20Reference))
  (|CallParentFunction OtherActor) ; This node is disabled and will not be called.\nDrag off pins to build functionality.
)

(event EventTick
  (params (DeltaSeconds :type Float%20%28single-precision%29))
  (|CallParentFunction DeltaSeconds) ; This node is disabled and will not be called.\nDrag off pins to build functionality.
)

(event EventCastAction
  (|CallParentFunction)
  (Default|CallOnActionStarted)
  (for _array_element (Variables|Default|GetTargets)
    (Niagara|SpawnSystematLocation "/Game/VFX/ElementalVFX/NS_NatureAura.NS_NatureAura" (+ (Transformation|GetActorLocation _array_element) "0.000000,0.000000,50.000000") "0, 0, 0" "0.500000,0.500000,0.500000"))
  (Audio|PlaySound2D "/Game/Audio/Magic_Spell_SFX_Pack_Vol1/Nature/cue/Nature_Magic_Spell_7-3_wav_Cue.Nature_Magic_Spell_7-3_wav_Cue" 1.0 1.0 0.0 0 0)
  (Timeline|Timeline PlayFromStart
    (:Finished
      (CallFunction|EndAction))
    (:Damage
      (for _array_element_2 (Variables|/Game/Blueprints/Units/BP_BaseUnit.BP_BaseUnit_C|GetAlliedUnits (Utilities|Array|Get(acopy) (Variables|Default|GetTargets)))
        (Default|DealDamage _array_element_2 2 (Utilities|Struct|BreakStruct_ActionData (Variables|Default|GetActionData)) (Variables|Default|GetActionUser) false)
        (Default|ApplyStatus _array_element_2 "/Game/Blueprints/Statuses/BP_StatusEntangle.BP_StatusEntangle_C" 2 false)))))

(fn ConstructionScript
  (|CallParentFunction))