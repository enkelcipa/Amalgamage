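; BP_Combine is an action that attempts to merge the acting unit with its first target.
; CastAction marks the target as acted in the game mode, plays a Niagara effect and sound, then calls Combine on the user.
; A timeline serves as the wait; if Combine succeeded, both units have statuses cleared and are destroyed, with a one-tick delay before the action ends.
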(event EventBeginPlay
  (|CallParentFunction) ; This node is disabled and will not be called.\nDrag off pins to build functionality.
)

(event Collision|EventActorBeginOverlap
  (params (OtherActor :type Actor%20Object%20Reference))
  (|CallParentFunction OtherActor) ; This node is disabled and will not be called.\nDrag off pins to build functionality.
)

(event EventTick
  (params (DeltaSeconds :type Float%20%28single-precision%29))
  (|CallParentFunction DeltaSeconds) ; This node is disabled and will not be called.\nDrag off pins to build functionality.
)

(event EventCastAction
  (bind _actionuser (Variables|Default|GetActionUser))
  (|CallParentFunction)
  (Default|CallOnActionStarted)
  (bind _output_get (Variables|Default|SetCombineTarget (Utilities|Array|Get(acopy) (Variables|Default|GetTargets))))
  (Utilities|Array|Add (Variables|/Game/Blueprints/Modes/GM_Battle.GM_Battle_C|GetActedUnits (Variables|Default|GetGameModeREF)) _output_get)
  (Niagara|SpawnSystematLocation "/Game/Basic_VFX/Niagara/NS_Basic_2.NS_Basic_2" (+ (Transformation|GetActorLocation _output_get) "0.000000,0.000000,50.000000") "0, 0, 0" "0.500000,0.500000,0.500000")
  (Audio|PlaySound2D "/Game/Audio/Magic_Spell_SFX_Pack_Vol1/Arcane/cue/Arcane_Magic_Spell_5-1_wav_Cue.Arcane_Magic_Spell_5-1_wav_Cue" 1.0 1.0 0.0 0 0)
  (bind _bsuccessful (Default|Combine (Variables|Default|GetActionUser) _output_get))
  (Timeline|Timeline PlayFromStart
    (:Finished
      (if _bsuccessful
        (Default|ClearAllStatuses (Variables|Default|GetCombineTarget))
        (Actor|DestroyActor (Variables|Default|GetCombineTarget))
        (Default|ClearAllStatuses _actionuser)
        (Actor|DestroyActor _actionuser)
        (Utilities|FlowControl|DelayUntilNextTick))
      (CallFunction|EndAction))))

(fn ConstructionScript
  (|CallParentFunction))