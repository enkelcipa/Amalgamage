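; BP_RainCloud is a combat action that casts a rain cloud on its first target.
; On cast it plays a wind spell sound and spawns the NS_Raincloud Niagara effect just above the target.
; A timeline's Damage event applies BP_StatusRainCloud to that target for a short duration, and the timeline's finish ends the action.
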(event EventCastAction
  ;[0.15 0.15 0.15 0.5] Cast Action Calls the Event of Action Started
  (|CallParentFunction)
  (Audio|PlaySound2D "/Game/Audio/Magic_Spell_SFX_Pack_Vol1/Wind/wav/Wind_Magic_Spell_1-1_wav.Wind_Magic_Spell_1-1_wav" 1.0 1.0 0.0 0 0)
  (Niagara|SpawnSystematLocation "/Game/VFX/ElementalVFX/NS_Raincloud.NS_Raincloud" (+ (Transformation|GetActorLocation (Utilities|Array|Get(acopy) (Variables|Default|GetTargets))) "0.000000,0.000000,50.000000"))
  (Timeline|Timeline PlayFromStart
    (:Finished
      (CallFunction|EndAction))
    (:Damage
      (Default|ApplyStatus (Utilities|Array|Get(acopy) (Variables|Default|GetTargets)) "/Game/Blueprints/Statuses/BP_StatusRainCloud.BP_StatusRainCloud_C" 2 false))))

(fn ConstructionScript
  (|CallParentFunction))