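; Depressurize combat action that damages its first target with a burst of steam effects and sound.
; CastAction plays a Timeline whose Damage event deals the hit and whose completion ends the action.
; If DealDamage returns true, the caster's mana is reduced through the game mode.
; Otherwise, the target's allies that pass an adjacency check against the targets receive a one-duration Blind status.
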(event EventCastAction
  ;[0.15 0.15 0.15 0.5] Cast Action Calls the Event of Action Started
  (|CallParentFunction)
  (Niagara|SpawnSystematLocation "/Game/VFX/ElementalVFX/NS_Steam.NS_Steam" (+ (Transformation|GetActorLocation (Variables|Default|GetActionUser)) "0.000000,0.000000,50.000000") "0.000000,180.000000,0.000000")
  (Audio|PlaySound2D "/Game/Audio/Magic_Spell_SFX_Pack_Vol1/General_Spells_and_Effects/cue/Negative_Magic_Effect_3-1_wav_Cue.Negative_Magic_Effect_3-1_wav_Cue" 1.0 1.0 0.0 0 0)
  (Timeline|Timeline Play
    (:Finished
      (CallFunction|EndAction))
    (:Damage
      (bind _blethal (Default|DealDamage (Utilities|Array|Get(acopy) (Variables|Default|GetTargets)) 18 (Utilities|Struct|BreakStruct_ActionData (Variables|Default|GetActionData)) (Variables|Default|GetActionUser) false))
      (if _blethal
        (Default|ModifyMana (Variables|Default|GetGameModeREF) false -15 (Variables|Default|GetActionUser))
        (else
          (for _array_element (Variables|/Game/Blueprints/Units/BP_BaseUnit.BP_BaseUnit_C|GetAlliedUnits (Utilities|Array|Get(acopy) (Variables|Default|GetTargets)))
            (bind _returnvalue (CallFunction|CheckAdjacentUnits _array_element (Variables|Default|GetTargets)))
            (if _returnvalue
              (Default|ApplyStatus _array_element "/Game/Blueprints/Statuses/BP_StatusBlind.BP_StatusBlind_C" 1 false))))))))

(fn ConstructionScript
  (|CallParentFunction))