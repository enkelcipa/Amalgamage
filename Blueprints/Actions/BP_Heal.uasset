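; BP_Heal is a castable action that heals the first target by a small flat amount plus a percentage of its max HP.
; CastAction calls the parent, signals the action's start, plays a sound and spawns a water aura Niagara effect above the target.
; A timeline paces the action, applying the healing on its event track named Damage and ending the action when it finishes.
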(event EventBeginPlay
  (|CallParentFunction) ; This node is disabled and will not be called.\nDrag off pins to build functionality.
)

(event Collision|EventActorBeginOverlap
  (params (OtherActor :type Actor%20Object%20Reference))
  (|CallParentFunction OtherActor) ; This node is disabled and will not be called.\nDrag off pins to build functionality.
)

(event EventTick
  (params (DeltaSeconds :type Float%20%28single-precision%29))
  (|CallParentFunction DeltaSeconds) ; This node is disabled and will not be called.\nDrag off pins to build functionality.
)

(event EventCastAction
  (bind _targets (Variables|Default|GetTargets))
  (bind _output (Utilities|Array|Get(acopy) _targets))
  ;[0.15 0.15 0.15 0.5] call parent fucntions
  (|CallParentFunction)
  (Default|CallOnActionStarted)
  (Audio|PlaySound2D "/Game/Audio/Magic_Spell_SFX_Pack_Vol1/General_Spells_and_Effects/cue/Positive_Magic_Effect_4-1_wav_Cue.Positive_Magic_Effect_4-1_wav_Cue" 1.0 1.0 0.0 0 0)
  (Niagara|SpawnSystematLocation "/Game/VFX/ElementalVFX/NS_WaterAura.NS_WaterAura" (+ (Transformation|GetActorLocation (Utilities|Array|Get(acopy) (Variables|Default|GetTargets))) "0.000000,0.000000,50.000000"))
  ;[0.15 0.15 0.15 0.5] timeline for vfx + end action
  (Timeline|Timeline PlayFromStart
    (:Finished
      (CallFunction|EndAction))
    (:Damage
      (Default|DealHealing _output (+ 5 (Math|Float|Round (* (Utilities|Struct|BreakStruct_UnitStats (Variables|/Game/Blueprints/Units/BP_BaseUnit.BP_BaseUnit_C|GetUnitStats _output)) 0.15)))))))

(fn ConstructionScript
  (|CallParentFunction))