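; Base actor for battle actions, giving them a shared start and end lifecycle.
; On BeginPlay it caches the GM_Battle game mode.
; CastAction fires OnActionStarted, then passes the mana cost from ActionData to the game mode's ModifyMana for the ActionUser.
; EndAction fires OnActionFinished, unbinds that dispatcher's listeners and destroys the actor.
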(event Custom|CastAction
  (Default|CallOnActionStarted)
  (Default|ModifyMana (Variables|Default|GetGameModeREF) false (.ManaCost (Utilities|Struct|BreakStruct_ActionData (Variables|Default|GetActionData))) (Variables|Default|GetActionUser)))

(event EventBeginPlay
  (bind _asgm_battle (Utilities|Casting|CastToGM_Battle (Game|GetGameMode)))
  (Variables|Default|SetGameModeREF _asgm_battle))

(event Collision|EventActorBeginOverlap
  (params (OtherActor :type Actor%20Object%20Reference)))

(event EventTick
  (params (DeltaSeconds :type Float%20%28single-precision%29)))

(fn ConstructionScript)

(fn EndAction
  (Default|CallOnActionFinished)
  (EventDispatchers|UnbindallEventsfromOnActionFinished)
  (Actor|DestroyActor))