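; Combat action that casts Overcharge on its first target, applying or re-triggering the Overcharge status.
; On cast it signals the action start, plays a lightning sound and spawns a Niagara effect at the target, then runs a timeline.
; The timeline's Damage event searches the target's attached actors for an existing status, calling its ApplyEffects if under three turns remain, or applies a new one if absent.
; The action ends when the timeline finishes.
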(event EventBeginPlay
  (|CallParentFunction) ; This node is disabled and will not be called.\nDrag off pins to build functionality.
)

(event Collision|EventActorBeginOverlap
  (params (OtherActor :type Actor%20Object%20Reference))
  (|CallParentFunction OtherActor) ; This node is disabled and will not be called.\nDrag off pins to build functionality.
)

(event EventTick
  (params (DeltaSeconds :type Float%20%28single-precision%29))
  (|CallParentFunction DeltaSeconds) ; This node is disabled and will not be called.\nDrag off pins to build functionality.
)

(event EventCastAction
  ;[0.15 0.15 0.15 0.5] calls parent functions
  (|CallParentFunction)
  (Default|CallOnActionStarted)
  (Audio|PlaySound2D "/Game/Audio/Magic_Spell_SFX_Pack_Vol1/Lightning/cue/Lightning_Magic_Spell_3-2_wav_Cue.Lightning_Magic_Spell_3-2_wav_Cue" 1.0 1.0 0.0 0 0)
  (Niagara|SpawnSystematLocation "/Game/Basic_VFX/Niagara/NS_Basic_9.NS_Basic_9" (+ (Transformation|GetActorLocation (Utilities|Array|Get(acopy) (Variables|Default|GetTargets))) ""))
  ;[0.15 0.15 0.15 0.5] timeline for vfx + end action
  (Timeline|Timeline PlayFromStart
    (:Finished
      (CallFunction|EndAction))
    (:Damage
      (for _array_element (Actor|GetAttachedActors (Utilities|Array|Get(acopy) (Variables|Default|GetTargets)) true false)
        (bind _asbp_status_overcharge (Utilities|Casting|CastToBP_StatusOvercharge _array_element))
        (Variables|Default|SetAs%20BP%20Status%20Overcharge _asbp_status_overcharge))
      (Utilities|IsValid (Variables|Default|GetAs%20BP%20Status%20Overcharge)
        (:Is%20Valid
          (if (< (Variables|/Game/Blueprints/Statuses/BP_BaseStatus.BP_BaseStatus_C|GetTurnsRemaining (Variables|Default|GetAs%20BP%20Status%20Overcharge)) 3)
            (Default|ApplyEffects (Variables|Default|GetAs%20BP%20Status%20Overcharge))))
        (:Is%20Not%20Valid
          (Default|ApplyStatus (Utilities|Array|Get(acopy) (Variables|Default|GetTargets)) "/Game/Blueprints/Statuses/BP_StatusOvercharge.BP_StatusOvercharge_C" 0 false))))))

(fn ConstructionScript
  (|CallParentFunction))