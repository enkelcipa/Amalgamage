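; BP_LavaGeyser is a combat action that erupts a lava geyser on the first target, applying damage-over-time and buffing its user.
; CastAction extends the parent cast with a spell sound, an earth-fire Niagara effect and a Timeline.
; The Timeline's Damage event applies the user's buff and the target's DoT, plus a shorter DoT on allies of the target that pass an adjacency check.
; The action ends when the Timeline finishes.
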(event EventCastAction
  ;[0.15 0.15 0.15 0.5] Cast Action Calls the Event of Action Started
  (|CallParentFunction)
  (Audio|PlaySound2D "/Game/Audio/Magic_Spell_SFX_Pack_Vol1/Nature/cue/Nature_Magic_Spell_4-2_wav_Cue.Nature_Magic_Spell_4-2_wav_Cue" 1.0 1.0 0.0 0 0)
  (Niagara|SpawnSystematLocation "/Game/VFX/ElementalVFX/NS_Earth+Fire.NS_Earth+Fire" (+ (Transformation|GetActorLocation (Utilities|Array|Get(acopy) (Variables|Default|GetTargets))) "0.000000,0.000000,50.000000") "0, 0, 0" "0.300000,0.300000,0.300000")
  (Timeline|Timeline PlayFromStart
    (:Finished
      (CallFunction|EndAction))
    (:Damage
      (Default|ApplyStatus (Variables|Default|GetActionUser) "/Game/Blueprints/Statuses/BP_StatusLavaGeyserBuff.BP_StatusLavaGeyserBuff_C" 2 false)
      (Default|ApplyStatus (Utilities|Array|Get(acopy) (Variables|Default|GetTargets)) "/Game/Blueprints/Statuses/BP_StatusLavaGeyserDoT.BP_StatusLavaGeyserDoT_C" 4 false)
      ;[0.15 0.15 0.15 0.5] Apply Status for adjacent units at a reduced duration
      (for _array_element (Variables|/Game/Blueprints/Units/BP_BaseUnit.BP_BaseUnit_C|GetAlliedUnits (Utilities|Array|Get(acopy) (Variables|Default|GetTargets)))
        (bind _returnvalue (CallFunction|CheckAdjacentUnits _array_element (Variables|Default|GetTargets)))
        (if _returnvalue
          (Default|ApplyStatus _array_element "/Game/Blueprints/Statuses/BP_StatusLavaGeyserDoT.BP_StatusLavaGeyserDoT_C" 2 false))))))

(fn ConstructionScript
  (|CallParentFunction))