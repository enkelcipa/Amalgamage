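; BP_Split is an action Blueprint that makes its user split, with a visual and sound effect.
; CastAction calls the parent, signals the action start, then spawns a Niagara effect slightly above the user and plays a 2D spell sound.
; A Timeline, with only its Finished output wired, acts as a delay before calling Split on the user and ending the action.
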(event EventBeginPlay
  (|CallParentFunction) ; This node is disabled and will not be called.\nDrag off pins to build functionality.
)

(event Collision|EventActorBeginOverlap
  (params (OtherActor :type Actor%20Object%20Reference))
  (|CallParentFunction OtherActor) ; This node is disabled and will not be called.\nDrag off pins to build functionality.
)

(event EventTick
  (params (DeltaSeconds :type Float%20%28single-precision%29))
  (|CallParentFunction DeltaSeconds) ; This node is disabled and will not be called.\nDrag off pins to build functionality.
)

(event EventCastAction
  (|CallParentFunction)
  (Default|CallOnActionStarted)
  (Niagara|SpawnSystematLocation "/Game/Basic_VFX/Niagara/NS_Basic_13.NS_Basic_13" (+ (Transformation|GetActorLocation (Variables|Default|GetActionUser)) "0.000000,0.000000,50.000000"))
  (Audio|PlaySound2D "/Game/Audio/Magic_Spell_SFX_Pack_Vol1/Arcane/cue/Arcane_Magic_Spell_4-3_wav_Cue.Arcane_Magic_Spell_4-3_wav_Cue" 1.0 1.0 0.0 0 0)
  (Timeline|Timeline PlayFromStart
    (:Finished
      (Default|Split (Variables|Default|GetActionUser))
      (CallFunction|EndAction))))

(fn ConstructionScript
  (|CallParentFunction))