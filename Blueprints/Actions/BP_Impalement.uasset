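; BP_Impalement is a combat action that hits its first target harder the lower that target's health is.
; On cast it plays a debris sound, spawns a metal Niagara effect above the target and runs a timeline whose Damage event deals the hit.
; Math expressions convert clamped health percentage into a linear bonus, reaching double base damage at the low-health floor.
; The action ends when the timeline finishes.
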(event EventCastAction
  (bind _targets (Variables|Default|GetTargets))
  (bind _output (Utilities|Array|Get(acopy) _targets))
  (bind _unitstats (Variables|/Game/Blueprints/Units/BP_BaseUnit.BP_BaseUnit_C|GetUnitStats _output))
  (bind (_maxhp _currenthp) (Utilities|Struct|BreakStruct_UnitStats _unitstats))
  (bind _returnvalue (Math|Conversions|ToFloat(Integer) _currenthp))
  (bind _returnvalue_2 (Math|Conversions|ToFloat(Integer) _maxhp))
  (bind _returnvalue_3 (|((CurrentHP/MaxHP)*100) _returnvalue _returnvalue_2))
  (bind _returnvalue_4 (Math|Float|Clamp(Float) _returnvalue_3 2e+01 1e+02))
  ;[0.15 0.15 0.15 0.5] Cast Action Calls the Event of Action Started
  (|CallParentFunction)
  (Audio|PlaySound2D "/Game/Audio/Magic_Spell_SFX_Pack_Vol1/Additional_and_Loops/cue/Debris_3_wav_Cue.Debris_3_wav_Cue" 1.0 1.0 0.0 0 0)
  (Niagara|SpawnSystematLocation "/Game/VFX/ElementalVFX/NS_Metal.NS_Metal" (+ (Transformation|GetActorLocation (Utilities|Array|Get(acopy) (Variables|Default|GetTargets))) "0.000000,0.000000,50.000000"))
  (Timeline|Timeline Play
    (:Finished
      (CallFunction|EndAction))
    (:Damage
      (if (== _returnvalue_4 1e+02)
        (Default|DealDamage _output (Math|Float|Round (Variables|Default|GetBase%20Damage)) (Utilities|Struct|BreakStruct_ActionData (Variables|Default|GetActionData)) (Variables|Default|GetActionUser) false)
        (else
          (Default|DealDamage _output (Math|Float|Round (|(BaseDamage*(1+(0.012500*(100-MissingHP)))) (Variables|Default|GetBase%20Damage) _returnvalue_4)) (Utilities|Struct|BreakStruct_ActionData (Variables|Default|GetActionData)) (Variables|Default|GetActionUser) false))))))

(fn ConstructionScript
  (|CallParentFunction))