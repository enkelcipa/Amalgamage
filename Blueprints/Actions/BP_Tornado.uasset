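; Tornado combat action that plays a wind sound and Niagara effect at the first target and damages that target's allied units.
; A timeline's Damage event raises the multiplier by 0.25 per actor attached to the target, expiring any that are BP_BaseStatus.
; The multiplied base damage is split evenly across the target's AlliedUnits, and the action ends when the timeline finishes.
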(event EventCastAction
  (bind _targets (Variables|Default|GetTargets))
  (bind _output (Utilities|Array|Get(acopy) _targets))
  (bind _alliedunits (Variables|/Game/Blueprints/Units/BP_BaseUnit.BP_BaseUnit_C|GetAlliedUnits _output))
  ;[0.15 0.15 0.15 0.5] Cast Action Calls the Event of Action Started
  (|CallParentFunction)
  (Audio|PlaySound2D "/Game/Audio/Magic_Spell_SFX_Pack_Vol1/Additional_and_Loops/cue/Wind_Loop_1_wav_Cue.Wind_Loop_1_wav_Cue" 1.0 1.0 0.0 0 0)
  (Niagara|SpawnSystematLocation "/Game/VFX/ElementalVFX/NS_Wind.NS_Wind" (+ (Transformation|GetActorLocation (Utilities|Array|Get(acopy) (Variables|Default|GetTargets))) "0.000000,0.000000,50.000000"))
  (Timeline|Timeline Play
    (:Finished
      (CallFunction|EndAction))
    (:Damage
      (for _array_element (Actor|GetAttachedActors _output true false)
        (Variables|Default|SetDamage%20Multiplier (+ (Variables|Default|GetDamage%20Multiplier) 0.25))
        (bind _asbp_base_status (Utilities|Casting|CastToBP_BaseStatus _array_element))
        (Default|StatusExpired _asbp_base_status))
      (for _array_element_2 _alliedunits
        (Default|DealDamage _array_element_2 (Math|Float|Round (/ (* (Variables|Default|GetBase%20Damage) (Variables|Default|GetDamage%20Multiplier)) (Utilities|Array|Length _alliedunits))) (Utilities|Struct|BreakStruct_ActionData (Variables|Default|GetActionData)) (Variables|Default|GetActionUser) false)))))

(fn ConstructionScript
  (|CallParentFunction))