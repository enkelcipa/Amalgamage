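; Thorns combat action that applies a short-lived thorns status to the character using it.
; On cast it plays a nature spell sound and spawns a nature-earth Niagara effect just above the first target.
; A timeline paces the action: its Damage event applies BP_StatusThorns to the action user, and completion ends the action.
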(event EventCastAction
  ;[0.15 0.15 0.15 0.5] Cast Action Calls the Event of Action Started
  (|CallParentFunction)
  (Audio|PlaySound2D "/Game/Audio/Magic_Spell_SFX_Pack_Vol1/Nature/cue/Nature_Magic_Spell_4-2_wav_Cue.Nature_Magic_Spell_4-2_wav_Cue" 1.0 1.0 0.0 0 0)
  (Niagara|SpawnSystematLocation "/Game/VFX/ElementalVFX/NS_Nature+Earth.NS_Nature+Earth" (+ (Transformation|GetActorLocation (Utilities|Array|Get(acopy) (Variables|Default|GetTargets))) "0.000000,0.000000,50.000000"))
  (Timeline|Timeline Play
    (:Finished
      (CallFunction|EndAction))
    (:Damage
      (Default|ApplyStatus (Variables|Default|GetActionUser) "/Game/Blueprints/Statuses/BP_StatusThorns.BP_StatusThorns_C" 2 false))))

(fn ConstructionScript
  (|CallParentFunction))