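; BP_ManaContainer is an actor that displays a mana fill level on a ball mesh with a numeric widget.
; BeginPlay applies a dynamic instance of MM_ManaTest to ManaBall.
; SetPercent drives the material's Fill% scalar and sends the value, scaled to a percentage, to the ManaNumbersWidget.
; SpawnIndicator currently does nothing, as its BP_ManaIndicator spawn is disconnected.
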(event Custom|SetPercent
  (params (0-1 :type Float%20%28double-precision%29))
  (Rendering|Material|SetScalarParameterValue (Variables|Default|GetMaterialREF) "Fill%" 0-1 :!class /Script/Engine.MaterialInstanceDynamic)
  (Class|BPIWidgetCom|ManaChanged(Message) (UserInterface|GetWidget (Variables|Default|GetMana%20Numbers%20Widget)) (* 0-1 1e+02)))

(event Custom|SpawnIndicator
  (params (ManaAdded :type Integer)))

(event EventBeginPlay
  (bind _returnvalue (Rendering|Material|CreateDynamicMaterialInstance "/Game/Materials/MM_ManaTest.MM_ManaTest" "None" "None" :!class /Script/Engine.KismetMaterialLibrary))
  (bind _output_get (Variables|Default|SetMaterialREF _returnvalue))
  (Rendering|Material|SetMaterial (Variables|Default|GetManaBall) 0 _output_get))

(event Collision|EventActorBeginOverlap
  (params (OtherActor :type Actor%20Object%20Reference)))

(event EventTick
  (params (DeltaSeconds :type Float%20%28single-precision%29)))

(fn ConstructionScript)