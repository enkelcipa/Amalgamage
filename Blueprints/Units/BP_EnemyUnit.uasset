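; Enemy unit Blueprint for action-based combat, extending a parent unit with AI-chosen actions and an animated hat.
; PrepareAction asks the ACAI component for an action and single target, queues them, and steps the unit forward via timeline before calling the parent.
; EndAction reverses that step.
; The construction script picks a helmet or slime crown from "Medium" or "Large" in the unit's name, while a second timeline animates the hat's height and yaw.
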(event Custom|MoveForwards
  (bind _defaultloc (Variables|Default|GetDefaultLoc))
  (bind _alpha (Timeline|Timeline_0 Play)
    (:Update
      (Transformation|SetActorLocation (Math|Vector|Lerp(Vector) _defaultloc (+ _defaultloc "-50.000000,0.000000,0.000000") _alpha) false false))))

(event Custom|MoveBackwards
  (bind _defaultloc (Variables|Default|GetDefaultLoc))
  (bind _alpha (Timeline|Timeline_0 Reverse)
    (:Update
      (Transformation|SetActorLocation (Math|Vector|Lerp(Vector) _defaultloc (+ _defaultloc "-50.000000,0.000000,0.000000") _alpha) false false))))

(event Custom|HatMovement
  (bind _hatmesh (Variables|Default|GetHatMesh))
  (bind (_direction _alphalocation _alpharotation) (Timeline|Timeline_1 PlayFromStart)
    (:Update
      (Transformation|SetRelativeLocation _hatmesh (Math|Vector|MakeVector 0.0 0.0 _alphalocation) false false)
      (Transformation|SetRelativeRotation _hatmesh (Math|Rotator|MakeRotator 0.0 0.0 _alpharotation) false false))))

(event EventBeginPlay
  (|CallParentFunction)
  (CallFunction|HatMovement))

(event Collision|EventActorBeginOverlap
  (params (OtherActor :type Actor%20Object%20Reference))
  (|CallParentFunction OtherActor) ; This node is disabled and will not be called.\nDrag off pins to build functionality.
)

(event EventTick
  (params (DeltaSeconds :type Float%20%28single-precision%29))
  (|CallParentFunction DeltaSeconds) ; This node is disabled and will not be called.\nDrag off pins to build functionality.
)

(event EventPrepareAction
  (Utilities|FlowControl|Delay 0.5)
  (Utilities|Array|Clear (Variables|Default|GetQueuedTargets))
  (bind (_chosen_action _target) (Default|AIBegin (Variables|Default|GetAC_AI) (Utilities|Struct|BreakStruct_UnitData (Variables|Default|GetUnitData)) (Variables|Default|GetEnemyUnits) (Variables|Default|GetAlliedUnits) self))
  (Variables|Default|SetQueuedAction (Utilities|GetClassDefaults _chosen_action))
  (Variables|Default|SetQueuedTargets (Utilities|Array|MakeArray _target))
  (CallFunction|MoveForwards)
  (|CallParentFunction))

(event EventEndAction
  (CallFunction|MoveBackwards)
  (Utilities|FlowControl|Delay 0.5)
  (|CallParentFunction))

(fn ConstructionScript
  (bind _hatmesh (Variables|Default|GetHatMesh))
  (bind _unitdata (Variables|Default|GetUnitData))
  (bind _name (Utilities|Struct|BreakStruct_UnitData _unitdata))
  (bind _returnvalue (Utilities|String|ToString(Text) _name))
  (|CallParentFunction)
  (if (Utilities|String|Contains _returnvalue "Medium")
    (Components|StaticMesh|SetStaticMesh _hatmesh "/Game/Meshes/HELMET.HELMET")
    (Transformation|SetRelativeScale3D _hatmesh "1.100000,1.100000,1.100000" :!label _label)
    (elif (Utilities|String|Contains _returnvalue "Large")
      (Components|StaticMesh|SetStaticMesh _hatmesh "/Game/Meshes/SlimeCrown.SlimeCrown")
      (goto _label))))