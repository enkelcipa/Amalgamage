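; BPC_StatHandler is a component that manages a unit's hit points in its UnitStats struct.
; ApplyDamage scales Amount by a Types map value, truncates and floors HP at zero, and returns from the loop body, so only the first entry applies.
; ApplyHealing caps HP at MaxHP.
; Both broadcast OnHitPointsModified with a healing flag, and damage reaching zero also fires OnKilled and returns true.
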(event EventBeginPlay)

(event EventTick
  (params (DeltaSeconds :type Float%20%28single-precision%29)))

(fn ApplyDamage
  (params (Amount :type Integer) (Types :type Map%20of%20eElement%20Enums%20to%20Reals :default "NewEnumerator0"))
  (bind _unitstats (Variables|Default|GetUnitStats))
  (bind _valuepin (Utilities|Map|ForEachLoop(Map) Types)
    (:then
      (Utilities|Struct|SetmembersinStruct_UnitStats _unitstats (Math|Integer|Max(Integer) (Math|Float|Truncate (- (Utilities|Struct|BreakStruct_UnitStats _unitstats) (* Amount _valuepin)))))
      (Default|CallOnHitPointsModified (Math|Integer|Max(Integer) (Math|Float|Truncate (- (Utilities|Struct|BreakStruct_UnitStats _unitstats) (* Amount _valuepin)))) false)
      (if (== (Math|Integer|Max(Integer) (Math|Float|Truncate (- (Utilities|Struct|BreakStruct_UnitStats _unitstats) (* Amount _valuepin)))) 0)
        (Default|CallOnKilled)
        (return true)
        (else
          (return false))))))

(fn ApplyHealing
  (params (Amount :type Integer))
  (bind _unitstats (Variables|Default|GetUnitStats))
  (bind (_currentaffinities _maxhp _currenthp) (Utilities|Struct|BreakStruct_UnitStats _unitstats))
  (bind _returnvalue (+ Amount _currenthp))
  (bind _returnvalue_2 (Math|Integer|Min(Integer) _maxhp _returnvalue))
  (Utilities|Struct|SetmembersinStruct_UnitStats _unitstats _returnvalue_2)
  (Default|CallOnHitPointsModified _returnvalue_2 true))