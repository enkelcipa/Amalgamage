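; BP_Spores is a combat action that infects its first target with spores while healing the user over time.
; Casting plays a sound, spawns the NS_Spores Niagara effect above the target and runs a timeline.
; The timeline's Damage event applies a damage-over-time status to the target and a heal-over-time status to the caster, both short-lived.
; When the timeline finishes, the action ends.
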(event EventCastAction
  ;[0.15 0.15 0.15 0.5] Cast Action Calls the Event of Action Started
  (|CallParentFunction)
  (Audio|PlaySound2D "/Game/Audio/Magic_Spell_SFX_Pack_Vol1/General_Spells_and_Effects/cue/Negative_Magic_Effect_4-2_wav_Cue.Negative_Magic_Effect_4-2_wav_Cue" 1.0 1.0 0.0 0 0)
  (Niagara|SpawnSystematLocation "/Game/VFX/ElementalVFX/NS_Spores.NS_Spores" (+ (Transformation|GetActorLocation (Utilities|Array|Get(acopy) (Variables|Default|GetTargets))) "0.000000,0.000000,50.000000"))
  (Timeline|Timeline Play
    (:Finished
      (CallFunction|EndAction))
    (:Damage
      (Default|ApplyStatus (Utilities|Array|Get(acopy) (Variables|Default|GetTargets)) "/Game/Blueprints/Statuses/BP_StatusSporesDoT.BP_StatusSporesDoT_C" 2 false)
      (Default|ApplyStatus (Variables|Default|GetActionUser) "/Game/Blueprints/Statuses/BP_StatusSporesHoT.BP_StatusSporesHoT_C" 2 false))))

(fn ConstructionScript
  (|CallParentFunction))