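; Fireball combat action that flies from the caster to the first target, exploding for fire effects and splash damage.
; CastAction calls the parent, then a timeline lerps the actor between the units.
; The timeline's Damage event plays sound and Niagara explosion, damages the target, then deals lesser damage to its adjacent allies, excluding the caster.
; The action ends when the timeline finishes.
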(event EventBeginPlay
  (|CallParentFunction) ; This node is disabled and will not be called.\nDrag off pins to build functionality.
)

(event Collision|EventActorBeginOverlap
  (params (OtherActor :type Actor%20Object%20Reference))
  (|CallParentFunction OtherActor) ; This node is disabled and will not be called.\nDrag off pins to build functionality.
)

(event EventTick
  (params (DeltaSeconds :type Float%20%28single-precision%29))
  (|CallParentFunction DeltaSeconds) ; This node is disabled and will not be called.\nDrag off pins to build functionality.
)

(event EventCastAction
  (bind _targets (Variables|Default|GetTargets))
  (bind _output (Utilities|Array|Get(acopy) _targets))
  (bind _returnvalue (Transformation|GetActorLocation _output))
  (bind _returnvalue_2 (+ _returnvalue "0.000000,0.000000,50.000000"))
  ;[0.15 0.15 0.15 0.5] calls parent functions
  (|CallParentFunction)
  (Default|CallOnActionStarted)
  (Audio|PlaySound2D "/Game/Audio/Magic_Spell_SFX_Pack_Vol1/General_Spells_and_Effects/cue/Magic_Cast_Whoosh_6-4_wav_Cue.Magic_Cast_Whoosh_6-4_wav_Cue" 1.0 1.0 0.0 0 0)
  ;[0.15 0.15 0.15 0.5] timeline for vfx + end action
  (bind _alpha (Timeline|Timeline Play)
    (:Update
      (Transformation|SetActorLocation (Math|Vector|Lerp(Vector) (+ (Transformation|GetActorLocation (Variables|Default|GetActionUser)) "0.000000,0.000000,50.000000") _returnvalue_2 _alpha) false false))
    (:Finished
      (CallFunction|EndAction))
    (:Damage
      (Audio|PlaySound2D "/Game/Audio/Magic_Spell_SFX_Pack_Vol1/Fire/cue/Fire_Magic_Spell_6-1_wav_Cue.Fire_Magic_Spell_6-1_wav_Cue" 1.0 1.0 0.0 0 0)
      (Niagara|SpawnSystematLocation "/Game/VFX/ElementalVFX/NS_Explosion.NS_Explosion" _returnvalue_2 "0, 0, 0" "0.500000,0.500000,0.500000")
      (Default|DealDamage _output 8 (Utilities|Struct|BreakStruct_ActionData (Variables|Default|GetActionData)) (Variables|Default|GetActionUser) false)
      (for _array_element (Variables|/Game/Blueprints/Units/BP_BaseUnit.BP_BaseUnit_C|GetAlliedUnits (Utilities|Array|Get(acopy) (Variables|Default|GetTargets)))
        ;[0.15 0.15 0.15 0.5] Action User cannot be adjacent to itself
        (if (not (== _array_element (Variables|Default|GetActionUser)))
          (bind _returnvalue_3 (CallFunction|CheckAdjacentUnits _array_element (Variables|Default|GetTargets)))
          (if _returnvalue_3
            (Utilities|Array|AddUnique (Variables|Default|GetAdjacentTargets) _array_element))))
      (for _array_element_2 (Variables|Default|GetAdjacentTargets)
        (Default|DealDamage _array_element_2 3 (Utilities|Struct|BreakStruct_ActionData (Variables|Default|GetActionData)) (Variables|Default|GetActionUser) false)))))

(fn ConstructionScript
  (|CallParentFunction))