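; Plasma Nova spell action that spends all the player's current mana to blast a target and its adjacent allies.
; Casting plays sound and an explosion effect, then a timeline triggers damage and ends the action.
; Damage scales MaxDamage by mana spent out of 100.
; Adjacent allies take the same damage with a PlasmaNova flag, and their HP is set to 1 when DealDamage returns true.
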(event EventCastAction
  (bind _gamemoderef (Variables|Default|GetGameModeREF))
  (bind _currentplayermana (Variables|/Game/Blueprints/Modes/GM_Battle.GM_Battle_C|GetCurrentPlayerMana _gamemoderef))
  (Audio|PlaySound2D "/Game/Audio/Magic_Spell_SFX_Pack_Vol1/Lightning/cue/Lightning_Magic_Spell_7-1_wav_Cue.Lightning_Magic_Spell_7-1_wav_Cue" 1.0 1.0 0.0 0 0)
  (Niagara|SpawnSystematLocation "/Game/VFX/ElementalVFX/NS_PlasmaExplosion.NS_PlasmaExplosion" (+ (Transformation|GetActorLocation (Utilities|Array|Get(acopy) (Variables|Default|GetTargets))) "0.000000,0.000000,50.000000"))
  (Utilities|Struct|SetmembersinStruct_ActionData (Variables|Default|GetActionData) _currentplayermana)
  (Variables|Default|SetMana%20Cost _currentplayermana)
  (|CallParentFunction)
  (Timeline|Timeline PlayFromStart
    (:Finished
      (CallFunction|EndAction))
    (:Damage
      (bind _output_get (Variables|Default|SetOutgoing%20Damage (Math|Float|Round (* (Math|Conversions|ToFloat(Integer) (Variables|Default|GetMax%20Damage)) (/ (Math|Conversions|ToFloat(Integer) (Variables|Default|GetMana%20Cost)) 1e+02)))))
      (Default|DealDamage (Utilities|Array|Get(acopy) (Variables|Default|GetTargets)) _output_get (Utilities|Struct|BreakStruct_ActionData (Variables|Default|GetActionData)) (Variables|Default|GetActionUser) false)
      (for _array_element (Variables|/Game/Blueprints/Units/BP_BaseUnit.BP_BaseUnit_C|GetAlliedUnits (Utilities|Array|Get(acopy) (Variables|Default|GetTargets)))
        (bind _returnvalue (CallFunction|CheckAdjacentUnits _array_element (Variables|Default|GetTargets)))
        (if _returnvalue
          (bind _blethal (Default|DealDamage _array_element (Variables|Default|GetOutgoing%20Damage) (Utilities|Struct|BreakStruct_ActionData (Variables|Default|GetActionData)) (Variables|Default|GetActionUser) true))
          (if _blethal
            (bind _structout (Utilities|Struct|SetmembersinStruct_UnitStats (Variables|/Game/Blueprints/Units/BP_BaseUnit.BP_BaseUnit_C|GetUnitStats _array_element) 1))
            (Default|CallOnHitPointsModified _array_element (.CurrentHP (Utilities|Struct|BreakStruct_UnitStats _structout)) (.MaxHP (Utilities|Struct|BreakStruct_UnitStats _structout)))))))))

(fn ConstructionScript
  (|CallParentFunction))