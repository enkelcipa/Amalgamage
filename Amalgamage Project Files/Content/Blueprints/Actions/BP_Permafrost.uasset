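; BP_Permafrost is a castable ice action that damages its first target and afflicts it with the Permafrost status.
; On cast it runs the parent action logic, plays a frost sound and spawns the NS_Ice Niagara effect just above the target.
; A Timeline paces the action: its Damage event deals damage using the action's damage types and applies the timed status, and its finish ends the action.
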(event EventBeginPlay
  (|CallParentFunction) ; This node is disabled and will not be called.\nDrag off pins to build functionality.
)

(event Collision|EventActorBeginOverlap
  (params (OtherActor :type Actor%20Object%20Reference))
  (|CallParentFunction OtherActor) ; This node is disabled and will not be called.\nDrag off pins to build functionality.
)

(event EventTick
  (params (DeltaSeconds :type Float%20%28single-precision%29))
  (|CallParentFunction DeltaSeconds) ; This node is disabled and will not be called.\nDrag off pins to build functionality.
)

(event EventCastAction
  (bind _targets (Variables|Default|GetTargets))
  (bind _output (Utilities|Array|Get(acopy) _targets))
  (|CallParentFunction)
  (Audio|PlaySound2D "/Game/Audio/Magic_Spell_SFX_Pack_Vol1/Frost/cue/Frost_Magic_Spell_5-4_wav_Cue.Frost_Magic_Spell_5-4_wav_Cue" 1.0 1.0 0.0 0 0)
  (Niagara|SpawnSystematLocation "/Game/VFX/ElementalVFX/NS_Ice.NS_Ice" (+ (Transformation|GetActorLocation (Utilities|Array|Get(acopy) (Variables|Default|GetTargets))) "0.000000,0.000000,50.000000"))
  (Timeline|Timeline Play
    (:Finished
      (CallFunction|EndAction))
    (:Damage
      (Default|DealDamage _output 10 (Utilities|Struct|BreakStruct_ActionData (Variables|Default|GetActionData)) (Variables|Default|GetActionUser) false)
      (Default|ApplyStatus _output "/Game/Blueprints/Statuses/BP_StatusPermafrost.BP_StatusPermafrost_C" 4 false))))

(fn ConstructionScript
  (|CallParentFunction))