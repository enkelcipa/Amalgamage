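; BP_SolarPower is an action that applies a Vulnerability status to its first target.
; On cast it plays a magic sound, spawns a Niagara effect above the target and starts a timeline.
; The timeline's Damage event applies the status, lasting one unit longer if the target is already in the game mode's ActedUnits list.
; The action ends when the timeline finishes.
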(event EventCastAction
  (bind _targets (Variables|Default|GetTargets))
  (bind _output (Utilities|Array|Get(acopy) _targets))
  ;[0.15 0.15 0.15 0.5] Cast Action Calls the Event of Action Started
  (|CallParentFunction)
  (Audio|PlaySound2D "/Game/Audio/Magic_Spell_SFX_Pack_Vol1/General_Spells_and_Effects/cue/Positive_Magic_Effect_6-3_wav_Cue.Positive_Magic_Effect_6-3_wav_Cue" 1.0 1.0 0.0 0 0)
  (Niagara|SpawnSystematLocation "/Game/Basic_VFX/Niagara/NS_Basic_10.NS_Basic_10" (+ (Transformation|GetActorLocation (Utilities|Array|Get(acopy) (Variables|Default|GetTargets))) "0.000000,0.000000,50.000000"))
  (Timeline|Timeline Play
    (:Finished
      (CallFunction|EndAction))
    (:Damage
      (if (Utilities|Array|ContainsItem (Variables|/Game/Blueprints/Modes/GM_Battle.GM_Battle_C|GetActedUnits (Variables|Default|GetGameModeREF)) _output)
        (Default|ApplyStatus _output "/Game/Blueprints/Statuses/BP_StatusVulnerability.BP_StatusVulnerability_C" 3 false)
        (else
          (Default|ApplyStatus _output "/Game/Blueprints/Statuses/BP_StatusVulnerability.BP_StatusVulnerability_C" 2 false))))))

(fn ConstructionScript
  (|CallParentFunction))