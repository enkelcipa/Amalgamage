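; Rain cloud status that doubles other statuses applied to its unit.
; On BeginPlay it binds to the unit's OnStatusApplied event, with DoubleStatus ignoring Rain Cloud and Shield and reapplying most others using class defaults and a RainCloud flag.
; Overcharge is special: an existing attached instance reruns its effects while its remaining turns are below a cap; otherwise, if none exists, one is applied without that flag.
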(event Custom|Double%20Status
  (params (Status%20Applied :type BP%20Base%20Status%20Class%20Reference))
  (if (not (== Status%20Applied "BP_StatusRainCloud_C"))
    (if (not (== Status%20Applied "/Game/Blueprints/Statuses/BP_StatusShield.BP_StatusShield_C"))
      (if (== Status%20Applied "/Game/Blueprints/Statuses/BP_StatusOvercharge.BP_StatusOvercharge_C")
        (for _array_element (Actor|GetAttachedActors (Variables|Default|GetUnit) true false)
          (bind _asbp_status_overcharge (Utilities|Casting|CastToBP_StatusOvercharge _array_element))
          (Variables|Default|SetOvercharge _asbp_status_overcharge))
        (Utilities|IsValid (Variables|Default|GetOvercharge)
          (:Is%20Valid
            (if (< (Variables|/Game/Blueprints/Statuses/BP_BaseStatus.BP_BaseStatus_C|GetTurnsRemaining (Variables|Default|GetOvercharge)) 3)
              (Default|ApplyEffects (Variables|Default|GetOvercharge))))
          (:Is%20Not%20Valid
            (Default|ApplyStatus (Variables|Default|GetUnit) "/Game/Blueprints/Statuses/BP_StatusOvercharge.BP_StatusOvercharge_C" 0 false)))
        (else
          (Default|ApplyStatus (Variables|Default|GetUnit) Status%20Applied (Utilities|GetClassDefaults Status%20Applied) true))))))

(event EventBeginPlay
  (|CallParentFunction)
  (EventDispatchers|BindEventtoOnStatusApplied (Variables|Default|GetUnit) (EventDispatchers|CreateEvent :!event Custom|Double%20Status)))

(event Collision|EventActorBeginOverlap
  (params (OtherActor :type Actor%20Object%20Reference))
  (|CallParentFunction OtherActor) ; This node is disabled and will not be called.\nDrag off pins to build functionality.
)

(event EventTick
  (params (DeltaSeconds :type Float%20%28single-precision%29))
  (|CallParentFunction DeltaSeconds) ; This node is disabled and will not be called.\nDrag off pins to build functionality.
)

(fn ConstructionScript
  (|CallParentFunction))