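; Blind status effect Blueprint that makes the afflicted unit's targeting random.
; On BeginPlay it binds an event to the unit's OnPreAbilitySpawn delegate.
; Its ApplyEffects event replaces the unit's QueuedTargets with a single random pick from its EnemyUnits.
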(event EventBeginPlay
  (|CallParentFunction)
  (EventDispatchers|BindEventtoOnPreAbilitySpawn (Variables|Default|GetUnit) (EventDispatchers|CreateEvent :!event ApplyEffects)))

(event Collision|EventActorBeginOverlap
  (params (OtherActor :type Actor%20Object%20Reference))
  (|CallParentFunction OtherActor) ; This node is disabled and will not be called.\nDrag off pins to build functionality.
)

(event EventTick
  (params (DeltaSeconds :type Float%20%28single-precision%29))
  (|CallParentFunction DeltaSeconds) ; This node is disabled and will not be called.\nDrag off pins to build functionality.
)

(event EventApplyEffects
  (bind _unit (Variables|Default|GetUnit))
  (Variables|/Game/Blueprints/Units/BP_BaseUnit.BP_BaseUnit_C|SetQueuedTargets _unit (Utilities|Array|MakeArray (.OutItem (Utilities|Array|Random (Variables|/Game/Blueprints/Units/BP_BaseUnit.BP_BaseUnit_C|GetEnemyUnits _unit))))))

(fn ConstructionScript
  (|CallParentFunction))