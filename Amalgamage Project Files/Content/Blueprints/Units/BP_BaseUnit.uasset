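; Base actor for an elemental unit in turn-based combat, taking its mesh, stats and actions from UnitData and showing HP, status, identity and target widgets.
; Queued actions spawn as actors that cast on targets, while statuses are spawned actors ticked through the unit.
; Damage is split across attack elements and base affinities, adjusted for weakness and resistance.
; Combine and Split merge or divide stats and statuses, broadcasting spawn and removal events for replacement units.
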(event Custom|SelectUnit
  (Rendering|SetVisibility (Variables|Default|GetArrow) true true)
  (Development|PrintString "Unit selected"))

(event Custom|DeselectUnit
  (Rendering|SetVisibility (Variables|Default|GetArrow) false true)
  (Development|PrintString "Unit deselected"))

(event Custom|EndAction
  (Default|CallOnTurnEnd))

(event Custom|Init
  (bind _unitdata (Variables|Default|GetUnitData))
  (bind _unitdata_2 (Variables|Default|GetUnitData))
  (bind (_baseaffinities _basehp _basespeed) (Utilities|Struct|BreakStruct_UnitData _unitdata_2))
  (bind _name (Utilities|Struct|BreakStruct_UnitData _unitdata))
  (Utilities|FlowControl|Sequence
    (:then_0
      (bind _returnvalue (UserInterface|CreateWidget "/Game/UI/WBP_UnitHP.WBP_UnitHP_C"))
      (bind _output_get (Variables|Default|SetHealthWidgetREF _returnvalue))
      (UserInterface|SetWidget (Variables|Default|GetHPWidget) _returnvalue)
      (Default|Init _output_get self))
    (:then_1
      (bind _returnvalue_2 (UserInterface|CreateWidget "/Game/UI/WBP_StatusHolder.WBP_StatusHolder_C"))
      (bind _output_get_2 (Variables|Default|SetStatusWidgetREF _returnvalue_2))
      (UserInterface|SetWidget (Variables|Default|GetStatusWidget) _output_get_2))
    (:then_3
      (bind _structout (Utilities|Struct|SetmembersinStruct_UnitStats (Variables|Default|GetUnitStats) _baseaffinities _basehp _basehp _basespeed))
      (Default|CallOnHitPointsModified (.CurrentHP (Utilities|Struct|BreakStruct_UnitStats _structout)) (.MaxHP (Utilities|Struct|BreakStruct_UnitStats _structout)))
      (Default|CallOnSpeedModified (.Speed (Utilities|Struct|BreakStruct_UnitStats _structout))))
    (:then_4
      (bind _returnvalue_3 (UserInterface|CreateWidget "/Game/UI/WBP_BlobIndicator.WBP_BlobIndicator_C"))
      (UserInterface|SetWidget (Variables|Default|GetBlobIndicatorWidget) _returnvalue_3)
      (Default|Init _returnvalue_3 _name (.CurrentAffinities (Utilities|Struct|BreakStruct_UnitStats (Variables|Default|GetUnitStats))) (Utilities|String|Contains (Utilities|String|ToString(Text) _name) "Enemy")))
    (:then_5
      (bind _returnvalue_4 (UserInterface|CreateWidget "/Game/UI/SpatialUI/WBP_Target.WBP_Target_C"))
      (UserInterface|SetWidget (Variables|Default|GetTargetWidget) _returnvalue_4)
      (Variables|Default|SetTargetWidgetREF _returnvalue_4)
      (Default|UpdateType _returnvalue_4 1.0))))

(event Custom|EnableDecals
  ;[0.15 0.15 0.15 0.5] Summoning Table Decal Cycle
  (Rendering|SetVisibility (Variables|Default|GetDecalLeftStrongerIcon) true false)
  (Rendering|SetVisibility (Variables|Default|GetDecalRightArrow) true false)
  (Rendering|SetVisibility (Variables|Default|GetDecalLeftArrow) true false)
  (Rendering|SetVisibility (Variables|Default|GetDecalRightWeakerIcon) true false))

(event Custom|Chosen
  ;[0.15 0.15 0.15 0.5] MainMenu
  (Variables|Default|SetChosenInMenu? true))

(event Custom|UnChosen
  ;[0.15 0.15 0.15 0.5] MainMenu
  (Variables|Default|SetChosenInMenu? false))

(event Custom|DisableDecals
  ;[0.15 0.15 0.15 0.5] Summoning Table Decal Cycle
  (Rendering|SetVisibility (Variables|Default|GetDecalLeftStrongerIcon) false false)
  (Rendering|SetVisibility (Variables|Default|GetDecalRightArrow) false false)
  (Rendering|SetVisibility (Variables|Default|GetDecalLeftArrow) false false)
  (Rendering|SetVisibility (Variables|Default|GetDecalRightWeakerIcon) false false))

(event EventBeginPlay
  (Utilities|FlowControl|Sequence
    (:then_0
      (CallFunction|Init)
      ;[0.1398 0.15 0.1194 0.5] Summoning Table Initial Decal Spawn
      (Rendering|Components|Decal|SetDecalMaterial (Variables|Default|GetDecalElemental) (Variables|Default|GetElementalDecalMaterial)))
    (:then_1
      (CallFunction|QueueAction "NewEnumerator0"))
    (:then_2
      (Variables|Default|SetDefaultLoc (Transformation|GetActorLocation)))))

(event Collision|EventActorBeginOverlap
  (params (OtherActor :type Actor%20Object%20Reference)))

(event EventOutlineOFF
  (Variables|Default|SetIsTargetted? false)
  (Development|SetHiddeninGame (Variables|Default|GetTargetWidget) true false))

(event EventTick
  (params (DeltaSeconds :type Float%20%28single-precision%29)))

(event EventIndicatorON
  (bind _defaultloc (Variables|Default|GetDefaultLoc))
  (Variables|Default|SetbIndicatorOn true)
  (Development|SetHiddeninGame (Variables|Default|GetIndicator) false false)
  (bind _alpha (Timeline|Timeline PlayFromStart)
    (:Update
      (Transformation|SetActorLocation (Math|Vector|Lerp(Vector) _defaultloc (+ _defaultloc "50.000000,0.000000,0.000000") _alpha) false false))))

(event EventAreYouTargetted
  (params (GameModeREF :type GM%20Battle%20Object%20Reference))
  (Default|GiveTargettedAnswer GameModeREF self (Variables|Default|GetIsTargetted?)))

(event EventPrepareAction
  (bind _unitdata (Variables|Default|GetUnitData))
  (bind _actions (Utilities|Struct|BreakStruct_UnitData _unitdata))
  (bind (_array_element _array_index) (Utilities|Array|ForEachLoopwithBreak _actions :!label _label)
    (:LoopBody
      (if (Utilities|Enum|Equal(Enum) (Variables|Default|GetQueuedAction) (Utilities|GetClassDefaults _array_element))
        (goto _label Break)))
    (:Completed
      (Default|CallOnPreAbilitySpawn)
      (CallFunction|ExecuteAction (Utilities|Array|Get(acopy) _actions _array_index) (Variables|Default|GetQueuedTargets))
      (Default|CallOnActionExecuted))))

(event EventOutlineon
  (params (Type :type Float%20%28double-precision%29))
  (if (not (Variables|Default|GetDead))
    (Variables|Default|SetIsTargetted? true)
    (Default|UpdateType (Variables|Default|GetTargetWidgetREF) Type)
    (Development|SetHiddeninGame (Variables|Default|GetTargetWidget) false false)))

(event EventQueueAction
  (params (ActionType :type eActionType%20Enum :default "NewEnumerator0") (Targets :type Array%20of%20BP%20Base%20Unit%20Object%20References))
  (Variables|Default|SetQueuedAction ActionType)
  (Variables|Default|SetQueuedTargets Targets))

(event EventIndicatorOFF
  (bind _defaultloc (Variables|Default|GetDefaultLoc))
  (if (Variables|Default|GetbIndicatorOn)
    (Development|SetHiddeninGame (Variables|Default|GetIndicator) true false)
    (Variables|Default|SetbIndicatorOn false)
    (bind _alpha (Timeline|Timeline ReverseFromEnd)
      (:Update
        (Transformation|SetActorLocation (Math|Vector|Lerp(Vector) _defaultloc (+ _defaultloc "50.000000,0.000000,0.000000") _alpha) false false)))))

(fn ConstructionScript
  (bind _cube (Variables|Default|GetCube))
  (bind _unitdata (Variables|Default|GetUnitData))
  (bind (_name _baseaffinities _mesh _material) (Utilities|Struct|BreakStruct_UnitData _unitdata))
  (Components|StaticMesh|SetStaticMesh _cube _mesh)
  (Rendering|Material|SetMaterial _cube 0 _material)
  (Rendering|Material|SetMaterial (Variables|Default|GetCube) 1 "/Game/Materials/MM_Transparent.MM_Transparent"))

(fn ExecuteAction
  (params (ActionClass :type BP%20Base%20Action%20Class%20Reference) (Targets :type Array%20of%20BP%20Base%20Unit%20Object%20References))
  (bind _returnvalue (Game|SpawnActorfromClass ActionClass (Transformation|GetActorTransform) "Undefined" "MultiplyWithRoot" 0 self Targets 0))
  (Default|CastAction _returnvalue)
  (EventDispatchers|BindEventtoOnActionFinished _returnvalue (EventDispatchers|CreateEvent :!event Custom|EndAction)))

(fn DealDamage
  (params (Amount :type Integer) (Types :type Map%20of%20eElement%20Enums%20to%20Reals :default "NewEnumerator0") (Caster :type BP%20Base%20Unit%20Object%20Reference) (Plasma%20Nova? :type Boolean))
  (bind _unitdata (Variables|Default|GetUnitData))
  (bind _unitstats (Variables|Default|GetUnitStats))
  (bind _baseaffinities (Utilities|Struct|BreakStruct_UnitData _unitdata))
  (bind (_maxhp _currenthp) (Utilities|Struct|BreakStruct_UnitStats _unitstats))
  (LocalVariables|SetTotal%20Incoming%20DMG 0)
  (Utilities|IsValid Caster
    (:Is%20Valid
      (Default|CallOnDealDamage Caster Amount))
    (:Is%20Not%20Valid
      _))
  (if (Utilities|Struct|BreakStruct_UnitStats (Variables|Default|GetUnitStats))
    (Default|CallOnHitBlocked)
    (else
      (Utilities|FlowControl|Sequence
        (:then_0
          (bind _keys (Utilities|Map|Keys Types))
          (for _array_element _keys
            (for _array_element_2 _baseaffinities
              (LocalVariables|SetDamage%20Multiplier 1.0)
              (LocalVariables|SetTotal%20Incoming%20DMG (+ (LocalVariables|GetTotal%20Incoming%20DMG) (Math|Float|Ceil (* (/ (/ Amount (Utilities|Array|Length _keys)) (Utilities|Array|Length _baseaffinities)) (+ (LocalVariables|GetDamage%20Multiplier) (Utilities|Select :Index (Math|Conversions|ToInteger(Boolean) (.Resistance (CallFunction|CompareElements _array_element _array_element_2))) :Option%200 0.0 :Option%201 -0.25) (Utilities|Select :Index (Math|Conversions|ToInteger(Boolean) (.Weakness (CallFunction|CompareElements _array_element _array_element_2))) :Option%200 0.0 :Option%201 0.25))))))
              (Game|SpawnActorfromClass "/Game/UI/SpatialUI/BP_DamageIndicator.BP_DamageIndicator_C" (Math|Transform|MakeTransform (+ (.location (Transformation|GetActorTransform)) (* (Math|Random|RandomUnitVector) 1e+01)) "0, 0, 0" "1.000000,1.000000,1.000000") "Undefined" "MultiplyWithRoot" 0 (Math|Float|Ceil (* (/ (/ Amount (Utilities|Array|Length _keys)) (Utilities|Array|Length _baseaffinities)) (+ (LocalVariables|GetDamage%20Multiplier) (Utilities|Select :Index (Math|Conversions|ToInteger(Boolean) (.Resistance (CallFunction|CompareElements _array_element _array_element_2))) :Option%200 0.0 :Option%201 -0.25) (Utilities|Select :Index (Math|Conversions|ToInteger(Boolean) (.Weakness (CallFunction|CompareElements _array_element _array_element_2))) :Option%200 0.0 :Option%201 0.25)))) _array_element false 0))))
        (:then_1
          (Utilities|Struct|SetmembersinStruct_UnitStats (Variables|Default|GetUnitStats) (Math|Integer|Max(Integer) (- (Utilities|Struct|BreakStruct_UnitStats (Variables|Default|GetUnitStats)) (LocalVariables|GetTotal%20Incoming%20DMG))))
          (Default|CallOnHitPointsModified _currenthp _maxhp)
          (if (<= _currenthp 0)
            (if Plasma%20Nova?
              (return true)
              (else
                (Variables|Default|SetDead true)
                (Default|CallOnKilled self)
                (return true)))
            (else
              (return false))))))))

(fn DealHealing
  (params (Amount :type Integer))
  (bind _unitstats (Variables|Default|GetUnitStats))
  (bind (_maxhp _currenthp) (Utilities|Struct|BreakStruct_UnitStats _unitstats))
  (bind _structout (Utilities|Struct|SetmembersinStruct_UnitStats (Variables|Default|GetUnitStats) (Math|Integer|Min(Integer) _maxhp (+ Amount _currenthp))))
  (Default|CallOnHitPointsModified (.CurrentHP (Utilities|Struct|BreakStruct_UnitStats _structout)) (.MaxHP (Utilities|Struct|BreakStruct_UnitStats _structout)))
  (Game|SpawnActorfromClass "/Game/UI/SpatialUI/BP_DamageIndicator.BP_DamageIndicator_C" (Transformation|GetActorTransform) "Undefined" "MultiplyWithRoot" 0 Amount "NewEnumerator0" true 0))

(fn ModifySpeed
  (params (Amount :type Integer))
  (bind _unitstats (Variables|Default|GetUnitStats))
  (bind _speed (Utilities|Struct|BreakStruct_UnitStats _unitstats))
  (bind _returnvalue (- _speed Amount))
  (Utilities|Struct|SetmembersinStruct_UnitStats (Variables|Default|GetUnitStats) _returnvalue)
  (Default|CallOnSpeedModified _returnvalue)
  (return (> Amount 0)))

(fn ChangePosition
  (params (NewPosition :type Integer))
  (Default|CallOnPositionSwapped NewPosition self))

(fn ModifyMana
  (params (Amount :type Integer))
  (if (not (Variables|Default|GetDead))
    (Game|SpawnActorfromClass "/Game/UI/SpatialUI/BP_ManaIndicator.BP_ManaIndicator_C" (Math|Transform|MakeTransform (+ (Transformation|GetActorLocation) "0.000000,0.000000,50.000000") "0, 0, 0" "1.000000,1.000000,1.000000") "Undefined" "MultiplyWithRoot" 0 Amount 0)))

(fn ApplyStatus
  (params (Class :type BP%20Base%20Status%20Class%20Reference) (Duration :type Integer) (Rain%20Cloud? :type Boolean))
  (bind _returnvalue (Game|SpawnActorfromClass Class (Transformation|GetActorTransform) "Undefined" "MultiplyWithRoot" 0 self Duration 0))
  (Utilities|Array|Add (Variables|Default|GetActiveStatuses) _returnvalue)
  (if (not Rain%20Cloud?)
    (Default|CallOnStatusApplied Class)
    (return _returnvalue)))

(fn TickStatuses
  (for _array_element (Variables|Default|GetActiveStatuses)
    (Utilities|IsValid _array_element
      (:Is%20Valid
        (Default|TickStatus _array_element)))))

(fn ClearAllStatuses
  (for _array_element (Variables|Default|GetActiveStatuses)
    (Utilities|IsValid _array_element
      (:Is%20Valid
        (Default|StatusExpired _array_element)))))

(fn Combine
  (params (TargetUnit :type BP%20Base%20Unit%20Object%20Reference))
  (bind _unitstats (Variables|BP_BaseUnit_C|GetUnitStats TargetUnit))
  (bind _unitstats_2 (Variables|Default|GetUnitStats))
  (bind (_currentaffinities _maxhp _currenthp _speed _attackmodifier _defensemodifier _binvincible) (Utilities|Struct|BreakStruct_UnitStats _unitstats))
  (bind (_currentaffinities_2 _maxhp_2 _currenthp_2 _speed_2 _attackmodifier_2 _defensemodifier_2 _binvincible_2) (Utilities|Struct|BreakStruct_UnitStats _unitstats_2))
  (bind _output (Utilities|Array|Get(acopy) _currentaffinities))
  (bind _output_2 (Utilities|Array|Get(acopy) _currentaffinities_2))
  (bind (_x _y) (CallFunction|ElementstoComboCoords _output _output_2))
  (Variables|BP_BaseUnit_C|SetDead TargetUnit true)
  (Variables|Default|SetDead true)
  (if (Math|Boolean|ORBoolean (> (Utilities|Array|Length _currentaffinities) 1) (> (Utilities|Array|Length _currentaffinities_2) 1) (Utilities|Enum|Equal(Enum) _output _output_2))
    (return false)
    (else
      (LocalVariables|SettCombinedStats (Utilities|Struct|MakeStruct_UnitStats (Utilities|Array|MakeArray _output _output_2) (+ _maxhp _maxhp_2) (+ _currenthp _currenthp_2) (+ _speed_2 _speed) (/ (+ _attackmodifier _attackmodifier_2) 2.0) (/ (+ _defensemodifier _defensemodifier_2) 2.0) (or _binvincible _binvincible_2)))
      (bind _effects_to_add (CallFunction|GetCombineStatus' (Variables|Default|GetActiveStatuses)))
      (LocalVariables|SettEffectsToAdd _effects_to_add)
      (bind _effects_to_add_2 (CallFunction|GetCombineStatus' (Variables|BP_BaseUnit_C|GetActiveStatuses TargetUnit)))
      (bind (_keypin _valuepin) (Utilities|Map|ForEachLoop(Map) _effects_to_add_2)
        (:then
          (Utilities|Map|Add (LocalVariables|GettEffectsToAdd) _keypin _valuepin))
        (:CompletedPin
          (Default|CallOnSpawnSignal (CallFunction|GetNamefromComboCoords (Math|Vector2D|MakeVector2D _x _y)) (Variables|BP_BaseUnit_C|GetPosition TargetUnit) (LocalVariables|GettCombinedStats) true false (LocalVariables|GettEffectsToAdd) (Utilities|Array|Get(acopy) (Utilities|Struct|BreakStruct_UnitStats (Variables|Default|GetUnitStats))) (Utilities|Array|Get(acopy) (Utilities|Struct|BreakStruct_UnitStats (Variables|BP_BaseUnit_C|GetUnitStats TargetUnit))) true)
          (Default|CallOnUnitRemoved self)
          (Default|CallOnUnitRemoved TargetUnit)
          (return true))))))

(fn Split
  (bind _self self)
  (bind _unitstats (Variables|Default|GetUnitStats))
  (bind (_currentaffinities _maxhp _currenthp _speed _attackmodifier _defensemodifier _binvincible) (Utilities|Struct|BreakStruct_UnitStats _unitstats))
  (Variables|Default|SetDead true)
  ;[0.15 0.15 0.15 0.5] Get the names of the units to spawn
  (for _index (range 0 1)
    (Utilities|Array|Add (LocalVariables|GetUnits%20to%20Spawn) (Utilities|String|StringToName (Utilities|String|Append "Blob" (Utilities|String|EnumtoString (Utilities|Array|Get(acopy) (Utilities|Struct|BreakStruct_UnitStats (Variables|Default|GetUnitStats)) _index))))))
  ;[0.15 0.15 0.15 0.5] Get the stats of the units to spawn
  (for _index_2 (range 0 1)
    (Utilities|Array|Add (LocalVariables|GetUnit%20Stats) (Utilities|Struct|MakeStruct_UnitStats (Utilities|Array|MakeArray (Utilities|Array|Get(acopy) _currentaffinities _index_2)) (Math|Float|Ceil (/ _maxhp 2)) (Math|Float|Ceil (/ _currenthp 2)) (Math|Float|Ceil (/ _speed 2)) _attackmodifier _defensemodifier _binvincible)))
  ;[0.15 0.15 0.15 0.5] Find open positions to spawn
  (bind _outactors (Actor|GetAllActorsOfClass "/Game/Blueprints/Units/BP_Blob.BP_Blob_C"))
  (for _array_element _outactors
    (if (not (== _array_element self))
      (Utilities|Array|RemoveItem (LocalVariables|GetPosition%20to%20Spawn) (Variables|BP_BaseUnit_C|GetPosition _array_element))))
  ;[0.15 0.15 0.15 0.5] Spawn the new units
  (for _index_3 (range 0 1)
    (Default|CallOnSpawnSignal (Utilities|Array|Get(acopy) (LocalVariables|GetUnits%20to%20Spawn) _index_3) (Utilities|Array|Get(acopy) (LocalVariables|GetPosition%20to%20Spawn) _index_3) (Utilities|Array|Get(acopy) (LocalVariables|GetUnit%20Stats) _index_3) true false (CallFunction|GetSplitStatus' (Variables|Default|GetActiveStatuses _self)) (Variables|Default|GetCombine%20Unit) (Variables|Default|GetSplit%20Unit) false))
  (CallFunction|ClearAllStatuses _self)
  (Default|CallOnUnitRemoved _self)
  (Actor|DestroyActor))

(fn FindLocationonTerrariumSurface
  (params (Loc :type Vector))
  (bind (_outhit _returnvalue) (Collision|LineTraceForObjects (+ Loc "0.000000,0.000000,50.000000") (- Loc "0.000000,0.000000,100.000000") (Utilities|Array|MakeArray "ObjectTypeQuery1") true 0 "ForDuration"))
  (if _returnvalue
    (return (.ImpactPoint (Collision|BreakHitResult _outhit)))))

(fn IsChoseninMenu?
  (return (Variables|Default|GetChosenInMenu?)))

(fn GetSplitStatus'
  (params (Active%20Status' :type Array%20of%20BP%20Base%20Status%20Object%20References))
  (Utilities|Map|Clear (LocalVariables|GetEffects%20to%20Add))
  (for _array_element Active%20Status'
    (Utilities|IsValid _array_element
      (:Is%20Valid
        (if (Utilities|Map|Contains (LocalVariables|GetEffects%20to%20Add) (Utilities|GetClass _array_element))
          (Utilities|Map|Add (LocalVariables|GetEffects%20to%20Add) (Utilities|GetClass _array_element) (Math|Float|Round (/ (+ (.Value (Utilities|Map|Find (LocalVariables|GetEffects%20to%20Add) (Utilities|GetClass _array_element))) (Variables|/Game/Blueprints/Statuses/BP_BaseStatus.BP_BaseStatus_C|GetTurnsRemaining _array_element)) 2.0)))
          (else
            (Utilities|Map|Add (LocalVariables|GetEffects%20to%20Add) (Utilities|GetClass _array_element) (Variables|/Game/Blueprints/Statuses/BP_BaseStatus.BP_BaseStatus_C|GetTurnsRemaining _array_element)))))))
  (return (LocalVariables|GetEffects%20to%20Add)))

(fn GetCombineStatus'
  (params (Active%20Status' :type Array%20of%20BP%20Base%20Status%20Object%20References))
  (Utilities|Map|Clear (LocalVariables|GetEffects%20to%20Add))
  (for _array_element Active%20Status'
    (Utilities|IsValid _array_element
      (:Is%20Valid
        (Utilities|Map|Add (LocalVariables|GetEffects%20to%20Add) (Utilities|GetClass _array_element) (Variables|/Game/Blueprints/Statuses/BP_BaseStatus.BP_BaseStatus_C|GetTurnsRemaining _array_element)))))
  (return (LocalVariables|GetEffects%20to%20Add)))