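; BP_ShieldCast is a cast action that gives shield status to the allied units of its first target.
; CastAction plays a sound and Niagara earth aura at that target, then runs a timeline whose Shield event applies the effect and whose finish ends the action.
; For each ally, it searches attached actors for BP_StatusShield and increments it, applying a new status first when no valid shield reference is held.
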(event EventBeginPlay
  (|CallParentFunction) ; This node is disabled and will not be called.\nDrag off pins to build functionality.
)

(event Collision|EventActorBeginOverlap
  (params (OtherActor :type Actor%20Object%20Reference))
  (|CallParentFunction OtherActor) ; This node is disabled and will not be called.\nDrag off pins to build functionality.
)

(event EventTick
  (params (DeltaSeconds :type Float%20%28single-precision%29))
  (|CallParentFunction DeltaSeconds) ; This node is disabled and will not be called.\nDrag off pins to build functionality.
)

(event EventCastAction
  (|CallParentFunction)
  (Default|CallOnActionStarted)
  (Audio|PlaySound2D "/Game/Audio/Magic_Spell_SFX_Pack_Vol1/General_Spells_and_Effects/cue/Positive_Magic_Effect_10-1_wav_Cue.Positive_Magic_Effect_10-1_wav_Cue" 1.0 1.0 0.0 0 0)
  (Niagara|SpawnSystematLocation "/Game/VFX/ElementalVFX/NS_EarthAura.NS_EarthAura" (+ (Transformation|GetActorLocation (Utilities|Array|Get(acopy) (Variables|Default|GetTargets))) "0.000000,0.000000,50.000000"))
  (Timeline|Timeline Play
    (:Finished
      (CallFunction|EndAction))
    (:Shield
      (for (_array_element _array_index) (Variables|/Game/Blueprints/Units/BP_BaseUnit.BP_BaseUnit_C|GetAlliedUnits (Utilities|Array|Get(acopy) (Variables|Default|GetTargets)))
        (for _array_element_2 (Actor|GetAttachedActors _array_element true false)
          (bind _asbp_status_shield (Utilities|Casting|CastToBP_StatusShield _array_element_2))
          (Variables|Default|SetAs%20BP%20Status%20Shield _asbp_status_shield))
        (Utilities|IsValid (Variables|Default|GetAs%20BP%20Status%20Shield)
          (:Is%20Valid
            (Default|IncrementShield (Variables|Default|GetAs%20BP%20Status%20Shield)))
          (:Is%20Not%20Valid
            (bind _applied_status_actor (Default|ApplyStatus (Utilities|Array|Get(acopy) (Variables|/Game/Blueprints/Units/BP_BaseUnit.BP_BaseUnit_C|GetAlliedUnits (Utilities|Array|Get(acopy) (Variables|Default|GetTargets))) _array_index) "/Game/Blueprints/Statuses/BP_StatusShield.BP_StatusShield_C" 0 false))
            (Default|IncrementShield _applied_status_actor)))))))

(fn ConstructionScript
  (|CallParentFunction))