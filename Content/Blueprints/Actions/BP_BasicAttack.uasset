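; BP_BasicAttack is a castable action that deals a unit's basic attack, typed by that unit's elemental affinities.
; On cast, it splits damage types evenly across the user's base affinities and writes them into ActionData.
; A Timeline's Damage event plays a sound, then spawns an element-colored Niagara effect per type above each target and deals damage.
; The action ends when the Timeline finishes.
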(event EventBeginPlay
  (|CallParentFunction) ; This node is disabled and will not be called.\nDrag off pins to build functionality.
)

(event Collision|EventActorBeginOverlap
  (params (OtherActor :type Actor%20Object%20Reference))
  (|CallParentFunction OtherActor) ; This node is disabled and will not be called.\nDrag off pins to build functionality.
)

(event EventTick
  (params (DeltaSeconds :type Float%20%28single-precision%29))
  (|CallParentFunction DeltaSeconds) ; This node is disabled and will not be called.\nDrag off pins to build functionality.
)

(event EventCastAction
  (bind _actiondata (Variables|Default|GetActionData))
  (bind _damagetypes (Utilities|Struct|BreakStruct_ActionData _actiondata))
  (|CallParentFunction)
  (CallFunction|UpdateDamageTypes)
  (Timeline|Timeline Play
    (:Finished
      (CallFunction|EndAction))
    (:Damage
      (Audio|PlaySound2D "/Game/Audio/Magic_Spell_SFX_Pack_Vol1/Arcane/cue/Arcane_Magic_Spell_2-1_wav_Cue.Arcane_Magic_Spell_2-1_wav_Cue" 1.0 1.0 0.0 0 0)
      (for _array_element (Variables|Default|GetTargets)
        (bind _keys (Utilities|Map|Keys _damagetypes))
        (for _array_element_2 _keys
          (Niagara|SpawnSystematLocation (Utilities|Select :Index _array_element_2 :NewEnumerator0 "/Game/VFX/TempFX/NS_TempBasicAttack.NS_TempBasicAttack" :NewEnumerator1 "/Game/VFX/TempFX/NS_TempBasicAttackBlue.NS_TempBasicAttackBlue" :NewEnumerator2 "/Game/VFX/TempFX/NS_TempBasicAttackYellow.NS_TempBasicAttackYellow" :NewEnumerator3 "/Game/VFX/TempFX/NS_TempBasicAttackGreen.NS_TempBasicAttackGreen" :NewEnumerator4 "/Game/VFX/TempFX/NS_TempBasicAttackPurple.NS_TempBasicAttackPurple") (+ (Transformation|GetActorLocation _array_element) "0.000000,0.000000,50.000000") "0, 0, 0" "0.500000,0.500000,0.500000"))
        (Default|DealDamage _array_element (Variables|Default|GetDamage) _damagetypes (Variables|Default|GetActionUser) false)))))

(fn ConstructionScript
  (|CallParentFunction))

(fn UpdateDamageTypes
  (bind _actionuser (Variables|Default|GetActionUser))
  (bind _unitdata (Variables|/Game/Blueprints/Units/BP_BaseUnit.BP_BaseUnit_C|GetUnitData _actionuser))
  (bind _baseaffinities (Utilities|Struct|BreakStruct_UnitData _unitdata))
  (for _array_element _baseaffinities
    (Utilities|Map|Add (LocalVariables|GettTypes) _array_element (/ 1 (Utilities|Array|Length _baseaffinities))))
  (Utilities|Struct|SetmembersinStruct_ActionData (Variables|Default|GetActionData) (LocalVariables|GettTypes)))