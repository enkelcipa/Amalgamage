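; Spores heal-over-time status Blueprint for battles that heals its Unit when its effects are applied.
; BeginPlay caches the GM_Battle game mode.
; ApplyEffects scales healing from the game mode's current enemy mana, dealing half of that mana times ManaDamage, rounded, as healing to the Unit.
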(event EventBeginPlay
  (|CallParentFunction)
  (bind _asgm_battle (Utilities|Casting|CastToGM_Battle (Game|GetGameMode)))
  (Variables|Default|SetGamemode%20REF _asgm_battle))

(event Collision|EventActorBeginOverlap
  (params (OtherActor :type Actor%20Object%20Reference))
  (|CallParentFunction OtherActor) ; This node is disabled and will not be called.\nDrag off pins to build functionality.
)

(event EventTick
  (params (DeltaSeconds :type Float%20%28single-precision%29))
  (|CallParentFunction DeltaSeconds) ; This node is disabled and will not be called.\nDrag off pins to build functionality.
)

(event EventApplyEffects
  (Default|DealHealing (Variables|Default|GetUnit) (Math|Float|Round (/ (* (Math|Conversions|ToFloat(Integer) (Variables|/Game/Blueprints/Modes/GM_Battle.GM_Battle_C|GetCurrentEnemyMana (Variables|Default|GetGamemode%20REF))) (Variables|Default|GetMana%20%25%20Damage)) 2.0))))

(fn ConstructionScript
  (|CallParentFunction))