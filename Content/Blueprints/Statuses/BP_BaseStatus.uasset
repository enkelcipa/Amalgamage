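; Base actor for turn-limited status effects on a unit, with empty apply, clear and shield-increment events for children to override.
; On BeginPlay it snaps to its Unit, adds a buff/debuff icon to the unit's status widget and broadcasts its remaining turns.
; TickStatus counts turns down and broadcasts changes; at zero the status clears effects, broadcasts expiry and destroys itself.
; ApplyEffects is left for children to call after parent BeginPlay.
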(event Custom|ApplyEffects)

(event Custom|Increment%20Shield)

(event Custom|StatusExpired
  (CallFunction|ClearEffects)
  (Default|CallOnStatusExpired)
  (Actor|DestroyActor))

(event Custom|ClearEffects)

(event Custom|TickStatus
  (bind _result (Math|Integer|DecrementInt (Variables|Default|GetTurnsRemaining))
    (:%20%20
      (Default|CallOnRemainingDurationModified _result)
      (if (== _result 0)
        (CallFunction|StatusExpired)))))

(event EventBeginPlay
  (bind _data (Variables|Default|GetData))
  (bind (_icon _bbuff) (Utilities|Struct|BreakStruct_StatusData _data))
  (Transformation|AttachActorToActor (Variables|Default|GetUnit) "None" "SnapToTarget" "SnapToTarget" "SnapToTarget" true)
  (bind _returnvalue (UserInterface|CreateWidget "/Game/UI/WBP_StatusIcon.WBP_StatusIcon_C" 0 _icon _bbuff))
  (Default|Init _returnvalue self)
  (Default|AddIcontoHolder (Variables|/Game/Blueprints/Units/BP_BaseUnit.BP_BaseUnit_C|GetStatusWidgetREF (Variables|Default|GetUnit)) _returnvalue)
  (Default|CallOnRemainingDurationModified (Variables|Default|GetTurnsRemaining)))

(event Collision|EventActorBeginOverlap
  (params (OtherActor :type Actor%20Object%20Reference)))

(event EventTick
  (params (DeltaSeconds :type Float%20%28single-precision%29)))

(fn ConstructionScript)