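; BP_StatusDoT is a damage-over-time status effect that hurts its affected unit each round.
; When TickStatus fires at the end of a round, it runs the parent tick and then ApplyEffects, which deals DamagePerTurn to the Unit using the DamageAffinity types.
; BeginPlay, overlap and Tick events are disabled stubs, so all behaviour runs through the status tick.
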(event EventBeginPlay
  (|CallParentFunction) ; This node is disabled and will not be called.\nDrag off pins to build functionality.
)

(event Collision|EventActorBeginOverlap
  (params (OtherActor :type Actor%20Object%20Reference))
  (|CallParentFunction OtherActor) ; This node is disabled and will not be called.\nDrag off pins to build functionality.
)

(event EventTick
  (params (DeltaSeconds :type Float%20%28single-precision%29))
  (|CallParentFunction DeltaSeconds) ; This node is disabled and will not be called.\nDrag off pins to build functionality.
)

(event EventApplyEffects
  (Default|DealDamage (Variables|Default|GetUnit) (Variables|Default|GetDamage%20per%20Turn) (Variables|Default|GetDamage%20Affinity) 0 false))

(event EventTickStatus
  ;[0.15 0.15 0.15 0.5] DoTs tick at the end of each round before the new round starts
  (|CallParentFunction)
  (CallFunction|ApplyEffects))

(fn ConstructionScript
  (|CallParentFunction))