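; Game instance that carries unit selection and level progress between the menu and battles.
; GetUnitNames converts selected elements to Blob unit names through a lookup map and returns them alongside the enemy names.
; Init creates per-level completion and score maps, which post-battle updates modify for the selected level.
; These updates also record previous stars, stars to fill, completed levels and return, replay and tutorial flags.
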(event EventInit
  (bind _levelscore (Variables|Default|GetLevelScore))
  (bind (_levelnumber _levelcompletion _levelscore_2) (Utilities|Struct|BreakStruct_LevelScore _levelscore))
  (Variables|Default|SetLevelCompletionMap (Utilities|Map|MakeMap _levelnumber _levelcompletion))
  (Variables|Default|SetLevelScoreMap (Utilities|Map|MakeMap _levelnumber _levelscore_2)))

(fn ElementstoNames
  (Utilities|Set|Clear (Variables|Default|GetPlayerUnitNames))
  (bind _valuepin (Utilities|Set|ForEachLoop(Set) (Variables|Default|GetElements))
    (:then
      (Utilities|Set|Add (Variables|Default|GetPlayerUnitNames) (.Value (Utilities|Map|Find (Utilities|Map|MakeMap "NewEnumerator0" "BlobFire" "NewEnumerator1" "BlobWater" "NewEnumerator2" "BlobEarth" "NewEnumerator3" "BlobNature" "NewEnumerator4" "BlobLightning") _valuepin)))
      (Development|PrintString (Utilities|String|ToString(Name) (.Value (Utilities|Map|Find (Utilities|Map|MakeMap "NewEnumerator0" "BlobFire" "NewEnumerator1" "BlobWater" "NewEnumerator2" "BlobEarth" "NewEnumerator3" "BlobNature" "NewEnumerator4" "BlobLightning") _valuepin)))))))

(fn GetUnitNames
  (CallFunction|ElementstoNames)
  (bind _result (Utilities|Set|ToArray (Variables|Default|GetPlayerUnitNames)))
  (return _result (Variables|Default|GetEnemyUnitNames)))

(fn UpdateLevelScore
  (params (ScoreToMenu :type Integer))
  (bind _levelscoremap (Variables|Default|GetLevelScoreMap))
  (bind _selectedlevel (Variables|Default|GetSelectedLevel))
  (bind (_value _returnvalue) (Utilities|Map|Find _levelscoremap _selectedlevel))
  (Variables|Default|SetPreviousStars _value)
  (if (>= ScoreToMenu _returnvalue)
    (Variables|Default|SetStarsToFill (- ScoreToMenu _value))
    (Utilities|Map|Add (Variables|Default|GetLevelScoreMap) (Variables|Default|GetSelectedLevel) ScoreToMenu)))

(fn UpdateLevelCompletion
  (params (IsVictorious :type Boolean))
  (bind _levelcompletionmap (Variables|Default|GetLevelCompletionMap))
  (Variables|Default|SetReturnFromBattle true)
  (Variables|Default|SetIsReplayed false)
  (if (!= (.Value (Utilities|Map|Find (Variables|Default|GetLevelCompletionMap) (Variables|Default|GetSelectedLevel))) IsVictorious)
    (Variables|Default|SetIsTutorialCompleted true)
    (Utilities|Map|Add _levelcompletionmap (Variables|Default|GetSelectedLevel) true)
    (Variables|Default|SetCompletedLevels (Utilities|Map|GetLastIndex _levelcompletionmap))
    (else
      (Variables|Default|SetIsReplayed true))))